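; Multiplayer GameInstance that manages online sessions through advanced session nodes: hosting, finding, joining and leaving servers.
; Hosting creates a session from ServerSettings, stores the settings, then opens the configured map as a listen server.
; Searches report through ServersFound on both success and failure.
; Quitting destroys the session and opens Lobby; network errors print the failure and quit the same way using the cached PlayerController.
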(event `Host Server`
  (params (PlayerController :type "PlayerController Object Reference") (ServerSettings :type "/Game/Blueprint/Networking/ServerSetting Structure"))
  (bind (_mapname _publicconnections _serversettings) (break `/Game/Blueprint/Networking/ServerSetting` ServerSettings))
  (bind _output_get (set `self.OwnerRef` PlayerController))
  (`CreateSessionCallbackProxyAdvanced.CreateAdvancedSession` _serversettings _output_get _publicconnections
    (:`OnSuccess`
      (set `self.ServerSettings` ServerSettings)
      (`GameplayStatics.OpenLevel` _mapname true "listen"))))

(event `Join Server`
  (params (PlayerController :type "PlayerController Object Reference") (SearchResult :type "BlueprintSessionResult Structure"))
  (bind _output_get (set `self.OwnerRef` PlayerController))
  (`JoinSessionCallbackProxy.JoinSession` _output_get SearchResult))

(event `Find Servers`
  (params (PlayerController :type "PlayerController Object Reference") (MaxResults :type Integer))
  (bind _results (`FindSessionsCallbackProxyAdvanced.FindSessionsAdvanced` PlayerController MaxResults false "AllServers")
    (:`OnSuccess`
      _)
    (:`OnFailure`
      _))
  (`self.Servers Found` _results))

(event `Quit To Lobby`
  (params (PlayerController :type "PlayerController Object Reference"))
  (`DestroySessionCallbackProxy.DestroySession` PlayerController
    (:`OnSuccess`
      (`GameplayStatics.OpenLevel` "Lobby"))))

(event `self.HandleNetworkError`
  (params (FailureType :type "ENetworkFailure Enum" :default "NetDriverAlreadyExists") (bIsServer :type Boolean))
  (bind _ownerref (`self.OwnerRef`))
  (`KismetSystemLibrary.PrintString` (`KismetStringLibrary.Concat_StrStr` (`|GetEnumeratorNameAsString` FailureType) " \n" (`KismetSystemLibrary.GetDisplayName` _ownerref)))
  (`self.Quit To Lobby` _ownerref))