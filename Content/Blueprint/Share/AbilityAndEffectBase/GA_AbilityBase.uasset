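; Base Gameplay Ability Blueprint that caches references to its avatar character and Ability System Component.
; On activation it fills CharacterPawn from the avatar as an ARTCharacterBase, then ASC as an ARTAbilitySystemComponent, casting only when the stored reference is invalid.
; A failed cast prints the ability's name with an error message.
; It contains no gameplay logic and does not end the ability itself.
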(event `self.K2_ActivateAbility`
  (`/Engine/EditorBlueprintResources/StandardMacros.IsValid` (`self.CharacterPawn`)
    (:`Is Valid`
      (`/Engine/EditorBlueprintResources/StandardMacros.IsValid` (`self.ASC`) :!label _label
        (:`Is Not Valid`
          (bind _asartability_system_component (cast `ARTAbilitySystemComponent` (`self.GetAbilitySystemComponentFromActorInfo`))
            (:`then`
              (set `self.ASC` _asartability_system_component))
            (:`CastFailed`
              (`KismetSystemLibrary.PrintString` (`KismetStringLibrary.Concat_StrStr` (`KismetSystemLibrary.GetDisplayName` self) " can't find AC")))))))
    (:`Is Not Valid`
      (bind _asartcharacter_base (cast `ARTCharacterBase` (`self.GetAvatarActorFromActorInfo`))
        (:`then`
          (set `self.CharacterPawn` _asartcharacter_base)
          (goto _label))
        (:`CastFailed`
          (`KismetSystemLibrary.PrintString` (`KismetStringLibrary.Concat_StrStr` (`KismetSystemLibrary.GetDisplayName` self) " can't find Avatar")))))))