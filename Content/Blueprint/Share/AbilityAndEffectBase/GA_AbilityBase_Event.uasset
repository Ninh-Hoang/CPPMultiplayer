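; Base gameplay ability for event-triggered abilities, caching the avatar character and its ability system component.
; On activation from an event, it lazily casts and stores CharacterPawn as ARTCharacterBase and ASC as ARTAbilitySystemComponent, stopping silently if a cast fails.
; CheckAndSetupCachables repeats this lazy setup as a callable function, printing the ability's name with an error when either cast fails.
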(event `self.K2_ActivateAbilityFromEvent`
  (params (EventData :type "GameplayEventData Structure (by ref)"))
  (`/Engine/EditorBlueprintResources/StandardMacros.IsValid` (`self.CharacterPawn`)
    (:`Is Valid`
      _)
    (:`Is Not Valid`
      (bind _asartcharacter_base (cast `ARTCharacterBase` (`self.GetAvatarActorFromActorInfo`)))
      (set `self.CharacterPawn` _asartcharacter_base)))
  (`/Engine/EditorBlueprintResources/StandardMacros.IsValid` (`self.ASC`)
    (:`Is Not Valid`
      (bind _asartability_system_component (cast `ARTAbilitySystemComponent` (`self.GetAbilitySystemComponentFromActorInfo`)))
      (set `self.ASC` _asartability_system_component))))