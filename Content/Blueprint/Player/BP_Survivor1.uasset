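; Player survivor Blueprint that runs a three-hit melee combo on the Confirm input through the Gameplay Ability System.
; It caches the ART ability system component shortly after possession, re-fetching it on input if invalid.
; Each press activates abilities by tag, advancing the chain within a short window after the last success, otherwise restarting at the first hit.
; Unconnected nodes that would add starter items to the inventory never run.
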(event `self.ReceiveBeginPlay`)

(event `self.ReceivePossessed`
  (params (NewController :type "Controller Object Reference"))
  (`KismetSystemLibrary.Delay` 0.1)
  (bind _asartability_system_component (cast `ARTAbilitySystemComponent` (`AbilitySystemBlueprintLibrary.GetAbilitySystemComponent` self)))
  (set `self.ASC` _asartability_system_component))

(event `InputAction|Confirm`
  (params (Key :type "Key Structure"))
  (:`Pressed`
    (`/Engine/EditorBlueprintResources/StandardMacros.IsValid` (`self.ASC`)
      (:`Is Valid`
        _)
      (:`Is Not Valid`
        (bind _asartability_system_component (cast `ARTAbilitySystemComponent` (`AbilitySystemBlueprintLibrary.GetAbilitySystemComponent` self)))
        (set `self.ASC` _asartability_system_component)))
    (if (> (- (`GameplayStatics.GetTimeSeconds`) (`self.TimeFromInput`)) 1.0)
      (bind _returnvalue (`AbilitySystemComponent.TryActivateAbilitiesByTag` (`self.ASC`) (`self.MeleeOne`) false :!label _label))
      (if _returnvalue
        (set `self.TimeFromInput` (`GameplayStatics.GetTimeSeconds`))
        (set `self.ComboChain` 0))
      (else
        (switch `int` (`self.ComboChain`)
          (:`0`
            (bind _returnvalue_2 (`AbilitySystemComponent.TryActivateAbilitiesByTag` (`self.ASC`) (`self.MeleeTwo`) false))
            (if _returnvalue_2
              (set `self.TimeFromInput` (`GameplayStatics.GetTimeSeconds`))
              (set `self.ComboChain` 1)))
          (:`1`
            (bind _returnvalue_3 (`AbilitySystemComponent.TryActivateAbilitiesByTag` (`self.ASC`) (`self.MeleeThree`) false))
            (if _returnvalue_3
              (set `self.TimeFromInput` (`GameplayStatics.GetTimeSeconds`))
              (set `self.ComboChain` 2)))
          (:`2`
            (goto _label)))))))

(fn `UserConstructionScript`)