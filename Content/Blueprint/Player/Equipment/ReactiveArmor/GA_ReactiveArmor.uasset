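; Gameplay ability for Reactive Armor equipment that stores up incoming attribute values, apparently damage, and releases them as a burst effect.
; On activation it caches the equipment, character and ASC, then sums each new value from an async attribute listener.
; At DamageBurstLimit it waits a frame, applies the Ability effect container with SetByCaller Data.Damage scaled from BaseDamage, then resets.
; An unused variant accumulates attribute decreases instead.
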(event `self.K2_ActivateAbility`
  (`self.CheckAndSetupCachables`)
  (set `self.CacheDamage` 0.0)
  (bind (_asynctaskproxy _attribute _newvalue) (`AsyncTaskAttributeChanged.ListenForAttributeChange` (`self.ASC`) (struct :`AttributeName` "Damage" :`Attribute` "/Script/ART.ARTCharacterAttributeSet:Damage"))
    (:`then`
      (set `self.ListenAttribute_Task` _asynctaskproxy))
    (:`OnAttributeChanged`
      (if (> _newvalue 0.1)
        (bind _output_get (set `self.CacheDamage` (+ (`self.CacheDamage`) _newvalue)))
        (`KismetSystemLibrary.PrintString` (`KismetStringLibrary.Conv_DoubleToString` _output_get))
        (if (>= _output_get (`self.DamageBurstLimit`))
          (`AT_WaitDelayOneFrame.WaitDelayOneFrame`
            (:`OnFinish`
              (bind _returnvalue (`self.MakeEffectContainerSpec` (struct :`TagName` "Ability")))
              (`AbilitySystemBlueprintLibrary.AssignTagSetByCallerMagnitude` (`|GetArrayItem` (`.TargetGameplayEffectSpecs` (break `ARTGameplayEffectContainerSpec` _returnvalue))) (struct :`TagName` "Data.Damage") (* (/ (`self.CacheDamage`) (`self.DamageBurstLimit`)) (`self.BaseDamage`)))
              (`self.ApplyEffectContainerSpec` _returnvalue)
              (set `self.CacheDamage` 0.0))))))))

(event `self.K2_OnEndAbility`
  (params (bWasCancelled :type Boolean))
  (`AsyncTaskAttributeChanged.EndTask` (`self.ListenAttribute_Task`)))