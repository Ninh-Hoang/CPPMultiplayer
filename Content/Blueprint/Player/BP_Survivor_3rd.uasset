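; BP_Survivor_3rd is a third-person survivor player Blueprint that hands out a starting loadout when play begins.
; BeginPlay adds items to the InventoryComponent by class: healing consumables, alcohol, several guns including a heal gun, and a sword.
; The remaining graph is unreached debug code that would print a dead state from the PlayerState's ability system tag or the current weapon's name.
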(event `self.ReceiveBeginPlay`
  (bind _inventorycomponent (`self.InventoryComponent`))
  (`InventoryComponent.TryAddItemFromClass` _inventorycomponent "/Game/Blueprint/ItemAndEquipment/Consumable/BP_Alcohol.BP_Alcohol_C" 5)
  (`InventoryComponent.TryAddItemFromClass` _inventorycomponent "/Game/Blueprint/ItemAndEquipment/Weapon/BP_Rifle.BP_Rifle_C" 1)
  (`InventoryComponent.TryAddItemFromClass` _inventorycomponent "/Game/Blueprint/ItemAndEquipment/Weapon/BP_Shotgun.BP_Shotgun_C" 1)
  (`InventoryComponent.TryAddItemFromClass` _inventorycomponent "/Game/Blueprint/ItemAndEquipment/Weapon/BP_TracerHealGun.BP_TracerHealGun_C" 1)
  (`InventoryComponent.TryAddItemFromClass` _inventorycomponent "/Game/Blueprint/ItemAndEquipment/Consumable/BP_Medkit.BP_Medkit_C" 5)
  (`InventoryComponent.TryAddItemFromClass` _inventorycomponent "/Game/Blueprint/ItemAndEquipment/Consumable/BP_Bandage.BP_Bandage_C" 5)
  (`InventoryComponent.TryAddItemFromClass` _inventorycomponent "/Game/Blueprint/ItemAndEquipment/Weapon/BP_Minigun.BP_Minigun_C" 1)
  (`InventoryComponent.TryAddItemFromClass` _inventorycomponent "/Game/Blueprint/ItemAndEquipment/Weapon/BP_Sword.BP_Sword_C" 1))

(fn `UserConstructionScript`)