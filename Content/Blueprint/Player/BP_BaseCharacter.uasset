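; Base player character that seeds starter inventory on the server, yaws its camera spring arm and draws debug damage hits.
; TestTrace deprojects the cursor onto a horizontal plane at actor height, traces to that point and opens a storage widget for any Storage hit.
; Construction passes camera, health and inventory components to InitializeComponents and limits scene capture to show this actor.
; Mouse aiming, movement and other UI prototypes are disconnected.
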(event `ServerIncreaseVariable`
  (`/Game/Blueprint/Framework/BP_GameStateBase.Increase Variable` (cast `/Game/Blueprint/Framework/BP_GameStateBase` (`GameplayStatics.GetGameState`) :!pure true)))

(event `InputAction|TestTrace`
  (params (Key :type "Key Structure"))
  (bind _returnvalue (`GameplayStatics.GetPlayerController` 0))
  (bind _asplayer_controller (cast `PlayerController` (`self.GetController`) :!pure true))
  (bind (_locationx _locationy) (`PlayerController.GetMousePosition` _asplayer_controller))
  (bind (_worldposition _worlddirection) (`GameplayStatics.DeprojectScreenToWorld` _asplayer_controller (`KismetMathLibrary.MakeVector2D` _locationx _locationy)))
  (bind (_t _intersection) (`KismetMathLibrary.LinePlaneIntersection` _worldposition (+ _worldposition (* _worlddirection 10000.0)) (`KismetMathLibrary.MakePlaneFromPointAndNormal` (`self.K2_GetActorLocation`) (`KismetMathLibrary.GetUpVector` (struct)))))
  ;[1 1 1] Open Storage
  (:`Pressed`
    (`KismetSystemLibrary.DrawDebugSphere` _intersection 50.0 12 (struct :`G` 1.0 :`B` 0.018589 :`A` 1.0) 1.0)
    (bind _outhit (`KismetSystemLibrary.LineTraceSingleForObjects` _worldposition _intersection (`|MakeArray` "ObjectTypeQuery4" :!type "EObjectTypeQuery Enum")))
    (bind (_bblockinghit _binitialoverlap _time _distance _location _impactpoint _normal _impactnormal _physmat _hitactor) (`GameplayStatics.BreakHitResult` _outhit))
    (`KismetSystemLibrary.PrintString` (`KismetSystemLibrary.GetDisplayName` _hitactor))
    (bind _asstorage (cast `Storage` _hitactor))
    (bind _returnvalue_2 (`|CreateWidget` "/Game/Blueprint/UI/WBP_StorageInventory.WBP_StorageInventory_C" _returnvalue _asstorage))
    (`UserWidget.AddToViewport` _returnvalue_2 0)
    (set `PlayerController.bShowMouseCursor` true _returnvalue)
    (`WidgetBlueprintLibrary.SetInputMode_UIOnlyEx` _returnvalue _returnvalue_2)))

(event `InputAxis|LookRight`
  (params (AxisValue :type "Float (single-precision)"))
  ;[1 1 1] Look Right, Need to move this to CPP
  (`SceneComponent.K2_AddRelativeRotation` (`self.CustomSpringArm`) (`KismetMathLibrary.MakeRotator` 0.0 0.0 AxisValue) false false))

(event `self.ReceiveBeginPlay`
  (`/Engine/EditorBlueprintResources/ActorMacros.Switch Has Authority`
    (:`Authority`
      (`InventoryComponent.TryAddItemFromClass` (`self.Inventory`) "/Game/Blueprint/Item/BP_Rifle_Item.BP_Rifle_Item_C" 1)
      (`InventoryComponent.TryAddItemFromClass` (`self.Inventory`) "/Game/Blueprint/Item/BP_Consumable_Alcohol.BP_Consumable_Alcohol_C" 3))))

(event `self.ReceiveTick`
  (params (DeltaSeconds :type "Float (single-precision)")))

(event `self.ReceivePointDamage`
  (params (Damage :type "Float (single-precision)") (DamageType :type "DamageType Object Reference") (HitLocation :type "Vector Structure") (HitNormal :type "Vector Structure") (HitComponent :type "PrimitiveComponent Object Reference") (BoneName :type Name) (ShotFromDirection :type "Vector Structure") (InstigatedBy :type "Controller Object Reference") (DamageCauser :type "Actor Object Reference") (HitInfo :type "HitResult Structure (by ref)"))
  ;[1 1 1] Draw Debug on Damaged
  (`KismetSystemLibrary.DrawDebugSphere` HitLocation 5.0 12 (struct :`R` 1.0 :`G` 0.087291 :`A` 1.0) 1.0 1.0)
  (`KismetSystemLibrary.DrawDebugString` HitLocation (`KismetStringLibrary.Conv_DoubleToString` Damage) null (struct :`R` 1.0 :`B` 0.018721 :`A` 1.0) 1.0))

(event `LookAtMouse`
  ;[1 1 1] Aiming Protoype
)

(fn `UserConstructionScript`
  (`self.InitializeComponents` (`self.CustomCamera`) (`self.CustomSpringArm`) (`self.SHealth`) (`self.Inventory`))
  (`KismetArrayLibrary.Array_AddUnique` (`SceneCaptureComponent.ShowOnlyActors` (`self.SceneCaptureComponent2D`)) self))