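; Base player controller Blueprint that creates and shows the player's inventory and notification UI.
; The OpenInventory input creates WBP_Inventory behind a validity check, adds it to the viewport, shows the cursor and switches to UI-only input focused on it.
; The CreateNotificationUI event lazily creates a cached WBP_NotificationStack widget and adds it to the viewport.
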(event `InputAction|OpenInventory`
  (params (Key :type "Key Structure"))
  (:`Pressed`
    (`/Engine/EditorBlueprintResources/StandardMacros.IsValid` null
      (:`Is Valid`
        _)
      (:`Is Not Valid`
        (bind _returnvalue (`|CreateWidget` "/Game/Blueprint/UI/WBP_Inventory.WBP_Inventory_C"))
        (set `self.InventoryWidget` _returnvalue)))
    (`UserWidget.AddToViewport` (`self.InventoryWidget`) 0)
    (set `self.bShowMouseCursor` true)
    (`WidgetBlueprintLibrary.SetInputMode_UIOnlyEx` self (`self.InventoryWidget`))))

(event `Create Notification UI`
  (`/Engine/EditorBlueprintResources/StandardMacros.IsValid` (`self.NotifiactionWidget`)
    (:`Is Valid`
      _)
    (:`Is Not Valid`
      (bind _returnvalue (`|CreateWidget` "/Game/Blueprint/Item/WBP_NotificationStack.WBP_NotificationStack_C"))
      (bind _output_get (set `self.NotifiactionWidget` _returnvalue))))
  (`UserWidget.AddToViewport` (`self.NotifiactionWidget`) 0)
  (`UserWidget.AddToViewport` _output_get 0))

(fn `UserConstructionScript`)