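; BP_Survivor is a player character Blueprint built on the Gameplay Ability System and an inventory component.
; BeginPlay seeds the inventory with a hard-coded loadout of consumables, weapons, armor and element items, and Possessed caches the custom ARTAbilitySystemComponent.
; On the authority, Tick prints debug text for Elec, Water and Electrocuted gameplay tags.
; Disconnected leftover nodes include melee ability activation by tag.
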(event `self.ReceiveBeginPlay`
  (bind _inventorycomponent (`self.InventoryComponent`))
  (`InventoryComponent.TryAddItemFromClass` _inventorycomponent "/Game/Blueprint/ItemAndEquipment/Consumable/BP_Alcohol.BP_Alcohol_C" 5)
  (`InventoryComponent.TryAddItemFromClass` _inventorycomponent "/Game/Blueprint/ItemAndEquipment/Consumable/BP_Medkit.BP_Medkit_C" 5)
  (`InventoryComponent.TryAddItemFromClass` _inventorycomponent "/Game/Blueprint/ItemAndEquipment/Consumable/BP_Bandage.BP_Bandage_C" 5)
  (`InventoryComponent.TryAddItemFromClass` _inventorycomponent "/Game/Blueprint/ItemAndEquipment/Weapon/BP_Staff.BP_Staff_C" 1)
  (`InventoryComponent.TryAddItemFromClass` _inventorycomponent "/Game/Blueprint/ItemAndEquipment/Equipment/BP_ReactiveArmor.BP_ReactiveArmor_C" 1)
  (`InventoryComponent.TryAddItemFromClass` _inventorycomponent "/Game/Blueprint/ItemAndEquipment/Weapon/BP_Minigun.BP_Minigun_C" 1)
  (`InventoryComponent.TryAddItemFromClass` _inventorycomponent "/Game/Blueprint/ItemAndEquipment/Consumable/ElementTestItem/BP_Electro.BP_Electro_C" 1)
  (`InventoryComponent.TryAddItemFromClass` _inventorycomponent "/Game/Blueprint/ItemAndEquipment/Consumable/ElementTestItem/BP_Hydro.BP_Hydro_C" 1))

(event `self.ReceivePossessed`
  (params (NewController :type "Controller Object Reference"))
  (bind _asartability_system_component (cast `ARTAbilitySystemComponent` (`AbilitySystemBlueprintLibrary.GetAbilitySystemComponent` self)))
  (set `self.ASC` _asartability_system_component))

(event `InputAction|Confirm`
  (params (Key :type "Key Structure")))

(event `self.ReceiveTick`
  (params (DeltaSeconds :type "Float (single-precision)"))
  (bind _returnvalue (`AbilitySystemBlueprintLibrary.GetAbilitySystemComponent` self))
  (`/Engine/EditorBlueprintResources/ActorMacros.Switch Has Authority`
    (:`Authority`
      (if (`GameplayTagAssetInterface.HasMatchingGameplayTag` _returnvalue (struct :`TagName` "State.Element.Elec"))
        (`KismetSystemLibrary.PrintString` "Elec" true true (struct :`G` 0.66 :`B` 1.0 :`A` 1.0) 0.0))
      (if (`GameplayTagAssetInterface.HasMatchingGameplayTag` _returnvalue (struct :`TagName` "State.Element.Water"))
        (`KismetSystemLibrary.PrintString` "Hydro" true true (struct :`G` 0.66 :`B` 1.0 :`A` 1.0) 0.0))
      (if (`GameplayTagAssetInterface.HasMatchingGameplayTag` _returnvalue (struct :`TagName` "State.Debuff.EleReact.Electrocuted"))
        (`KismetSystemLibrary.PrintString` "Electrocuted" true true (struct :`G` 0.66 :`B` 1.0 :`A` 1.0) 0.0)))))

(fn `UserConstructionScript`)