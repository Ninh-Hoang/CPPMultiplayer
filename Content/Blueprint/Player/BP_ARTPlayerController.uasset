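; Player controller that opens the inventory and attribute status screens and provides debug hotkeys.
; Each screen is created on first use, cached and added to the viewport with the cursor shown and UI-only input; both focus the Inventory widget.
; M, J, K and L run console commands for animation and ability-system debugging and simulated packet lag.
; An unconnected waypoint indicator test, spawning two marker actors, never runs.
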(event `Key|M`
  (params (Key :type "Key Structure"))
  (:`Pressed`
    (`KismetSystemLibrary.ExecuteConsoleCommand` "showdebug ANIMATION" null)))

(event `Key|J`
  (params (Key :type "Key Structure"))
  (:`Pressed`
    (`KismetSystemLibrary.ExecuteConsoleCommand` "Net PktLag=500" null)))

(event `Key|K`
  (params (Key :type "Key Structure"))
  (:`Pressed`
    (`KismetSystemLibrary.ExecuteConsoleCommand` "showdebug abilitysystem" null)))

(event `Key|L`
  (params (Key :type "Key Structure"))
  (:`Pressed`
    (`KismetSystemLibrary.ExecuteConsoleCommand` "AbilitySystem.Debug.NextCategory" null)))

(event `InputAction|OpenInventory`
  (params (Key :type "Key Structure"))
  (:`Pressed`
    (`/Engine/EditorBlueprintResources/StandardMacros.IsValid` (`self.Inventory`)
      (:`Is Valid`
        _)
      (:`Is Not Valid`
        (bind _returnvalue (`|CreateWidget` "/Game/Blueprint/UI/WBP_Inventory.WBP_Inventory_C"))
        (set `self.Inventory` _returnvalue)))
    (`UserWidget.AddToViewport` (`self.Inventory`) 0)
    (set `self.bShowMouseCursor` true)
    (`WidgetBlueprintLibrary.SetInputMode_UIOnlyEx` self (`self.Inventory`))))

(event `InputAction|Status`
  (params (Key :type "Key Structure"))
  (:`Pressed`
    (`/Engine/EditorBlueprintResources/StandardMacros.IsValid` (`self.AttributePreview`)
      (:`Is Valid`
        _)
      (:`Is Not Valid`
        (bind _returnvalue (`|CreateWidget` "/Game/Blueprint/UI/Player/UI_AttributeStatus.UI_AttributeStatus_C"))
        (set `self.AttributePreview` _returnvalue)))
    (`UserWidget.AddToViewport` (`self.AttributePreview`) 0)
    (set `self.bShowMouseCursor` true)
    (`WidgetBlueprintLibrary.SetInputMode_UIOnlyEx` self (`self.Inventory`))))

(event `self.ReceiveBeginPlay`)

(fn `UserConstructionScript`)