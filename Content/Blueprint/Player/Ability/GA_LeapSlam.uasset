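; Gameplay ability for a survivor's leap slam, currently only wired through its targeting step.
; On activation it casts the avatar to ARTSurvivor and starts a user-confirmed WaitTargetData task with a target actor class, passing a start location offset ahead of the character.
; Nothing handles the target data: commit, cancel and the alternative existing-actor targeting nodes are disconnected, and no leap or damage logic exists.
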(event `self.K2_ActivateAbility`
  (bind (_locationtype _literaltransform _sourceactor _sourcecomponent _sourceability _sourcesocketname) (break `GameplayAbilityTargetingLocationInfo` (`self.MakeTargetLocationInfoFromOwnerActor`)))
  (bind _asartsurvivor (cast `ARTSurvivor` (`self.GetAvatarActorFromActorInfo`)))
  (set `self.Character` _asartsurvivor)
  (`AbilityTask_WaitTargetData.WaitTargetData` "None" "UserConfirmed" (`self.TargetActor`) 0.0 0.0 999999.0 (struct :`Name` "PhysicsActor") true (make `GameplayAbilityTargetingLocationInfo` _locationtype (`KismetMathLibrary.MakeTransform` (+ (* (`Actor.GetActorForwardVector` (`self.Character`)) 200.0) (.location _literaltransform)) (.rotation _literaltransform) (.scale _literaltransform)) _sourceactor _sourcecomponent _sourceability _sourcesocketname) (struct) null))