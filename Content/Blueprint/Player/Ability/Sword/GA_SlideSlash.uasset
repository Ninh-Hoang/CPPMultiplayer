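; Gameplay ability for a greatsword slide attack that only runs while the character is sprinting, otherwise cancelling.
; After caching character, weapon and its melee trace actor, it waits a frame and plays the montage.
; The attack-start event opens a reusable-actor target data task, confirmed on each valid trace callback without ending.
; Each result applies GE_SlideSlash with set-by-caller damage; the LeapSlam impact cue is unwired.
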(event `self.K2_ActivateAbility`
  (bind _targetactor (`self.TargetActor`))
  (`self.SetupCachables`
    (:`Is Valid`
      ;[1 1 1] Blend Animation
      (if (`GameplayTagAssetInterface.HasMatchingGameplayTag` (`self.GetAbilitySystemComponentFromActorInfo`) (struct :`TagName` "State.Sprinting"))
        (`AT_WaitDelayOneFrame.WaitDelayOneFrame`
          (:`OnFinish`
            (bind (_asynctaskproxy _eventtag) (`AT_PlayMontageMeshWaitForEvent.PlayMontageForMeshAndWaitForEvent` "None" (`Character.Mesh` (`self.Character`)) "/Game/Blueprint/Animation/great_sword_slide_attack_Montage.great_sword_slide_attack_Montage" (struct :`GameplayTags` (struct :`(TagName` "Event.Montage.AttackStart") :`(TagName` "Event.Montage.AttackEnd"))) 1.5)
              (:`then`
                (set `self.MontageTask` _asynctaskproxy))
              (:`OnCompleted`
                (`self.K2_EndAbility` :!label _label))
              (:`OnBlendOut`
                (goto _label))
              (:`OnInterrupted`
                (`self.K2_CancelAbility` :!label _label_2))
              (:`OnCancelled`
                (goto _label_2))
              (:`EventReceived`
                (`GATA_MeleeWeaponTrace.Configure` :`self` _targetactor :`InMeleeWeaponActor` (`self.SourceWeapon`) :`InStartLocation` (make `GameplayAbilityTargetingLocationInfo` "LiteralTransform" (`KismetMathLibrary.Conv_VectorToTransform` (`Actor.K2_GetActorLocation` (`self.SourceWeapon`)))) :`InTraceProfile` (struct :`Name` "NoCollision") :`bInDebug` true)
                (add `GATA_MeleeWeaponTrace.ValidData` _targetactor (delegate `MeleeDataHandle`))
                (if (`BlueprintGameplayTagLibrary.MatchesTag` _eventtag (struct :`TagName` "Event.Montage.AttackStart"))
                  (bind (_asynctaskproxy_2 _data) (`AT_WaitTargetDataUsingActor.WaitTargetDataWithReusableActor` "Target" "CustomMulti" (`self.TargetActor`) true)
                    (:`then`
                      (set `self.WaitTargetDataTask` _asynctaskproxy_2))
                    (:`ValidData`
                      (`self.HandleTargetData` _data))
                    (:`Cancelled`
                      (`self.K2_EndAbility`)))
                  (else
                    (`self.ConfirmTaskByInstanceName` "Target" true)))))))
        (else
          (`self.K2_CancelAbility`))))))

(event `MeleeDataHandle`
  (`self.ConfirmTaskByInstanceName` "Target"))

(event `HandleTargetData`
  (params (Data :type "GameplayAbilityTargetDataHandle Structure"))
  (bind _returnvalue (`AbilitySystemBlueprintLibrary.AssignTagSetByCallerMagnitude` (`self.MakeOutgoingGameplayEffectSpec` "/Game/Blueprint/Player/Ability/Sword/GE_SlideSlash.GE_SlideSlash_C") (struct :`TagName` "Data.Damage") (`self.Damage`)))
  (`self.K2_ApplyGameplayEffectSpecToTarget` _returnvalue Data)
  (bind _returnvalue_2 (`AbilitySystemBlueprintLibrary.GetEffectContext` _returnvalue)))

(event `self.K2_OnEndAbility`
  (params (bWasCancelled :type Boolean))
  (bind _waittargetdatatask (`self.WaitTargetDataTask`))
  (`/Engine/EditorBlueprintResources/StandardMacros.IsValid` _waittargetdatatask
    (:`Is Valid`
      (`GameplayTask.EndTask` _waittargetdatatask))))