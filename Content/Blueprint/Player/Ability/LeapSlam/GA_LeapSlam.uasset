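; Leap Slam gameplay ability: plays the slam montage and damages targets found when the impact event fires.
; On impact, a cached, reusable sphere-trace TargetActor produces target data instantly, alongside a server task awaiting replicated client data.
; HandleTargetData applies a SetByCaller damage effect and executes the impact GameplayCue.
; The ability ends or cancels with the montage, and OnEndAbility stops the server wait task.
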(event `self.K2_ActivateAbility`
  (bind _targetactor (`self.TargetActor`))
  (`self.SetupCachebles`)
  (`AT_PlayMontageMeshWaitForEvent.PlayMontageForMeshAndWaitForEvent` "None" (`Character.Mesh` (`self.Character`)) "/Game/AnimStarterPack/MX_Animation/MT_leap_slam.MT_leap_slam" (struct :`GameplayTags` (struct :`(TagName` "Ability.LeapSlam.Impact"))) 1.5
    (:`OnCompleted`
      (`self.K2_EndAbility` :!label _label))
    (:`OnBlendOut`
      (goto _label))
    (:`OnInterrupted`
      (`self.K2_CancelAbility` :!label _label_2))
    (:`OnCancelled`
      (goto _label_2))
    (:`EventReceived`
      ;[1 1 1] Tell the Server to start waiting for replicated TargetData. Client simply returns from the Task's Activate(). If the player is the Server (Host), this won't do anything
      (bind (_asynctaskproxy _data) (`AT_ServerWaitForClientTargetData.ServerWaitForClientTargetData` "None")
        (:`then`
          (set `self.ServerWaitTargetDataTask` _asynctaskproxy)
          (`GATA_SphereTrace.Configure` :`self` _targetactor :`InStartLocation` (`self.MakeTargetLocationInfoFromOwnerActor`) :`InTraceProfile` (struct :`Name` "Pawn") :`bInShouldProduceTargetDataOnServer` true :`bInIgnoreSourceActor` true :`bInDebug` true :`InMaxRange` 0.0 :`InTraceSphereRadius` (`self.TraceSphereRadius`) :`InMaxHitResultsPerTrace` (`self.MaxTarget`))
          (bind (_asynctaskproxy_2 _data_2) (`AT_WaitTargetDataUsingActor.WaitTargetDataWithReusableActor` "None" "Instant" _targetactor true)
            (:`ValidData`
              (`self.HandleTargetData` _data_2))
            (:`Cancelled`
              (`self.K2_CancelAbility`))))
        (:`ValidData`
          (`self.HandleTargetData` _data))))))

(event `HandleTargetData`
  (params (TargetData :type "GameplayAbilityTargetDataHandle Structure"))
  (bind _returnvalue (`AbilitySystemBlueprintLibrary.AssignTagSetByCallerMagnitude` (`self.MakeOutgoingGameplayEffectSpec` "/Game/Blueprint/Player/Ability/LeapSlam/GE_LeapSlamDamage.GE_LeapSlamDamage_C") (struct :`TagName` "Data.Damage") (`self.LeapSlamDamage`)))
  (`self.K2_ApplyGameplayEffectSpecToTarget` _returnvalue TargetData)
  (bind _returnvalue_2 (`AbilitySystemBlueprintLibrary.GetEffectContext` _returnvalue))
  (`self.K2_ExecuteGameplayCueWithParams` (struct :`TagName` "GameplayCue.Ability.LeapSlam.Impact") (`AbilitySystemBlueprintLibrary.MakeGameplayCueParameters` 0.0 0.0 _returnvalue_2)))

(event `self.K2_OnEndAbility`
  (params (bWasCancelled :type Boolean))
  (bind _serverwaittargetdatatask (`self.ServerWaitTargetDataTask`))
  (`/Engine/EditorBlueprintResources/StandardMacros.IsValid` _serverwaittargetdatatask
    (:`Is Valid`
      (`GameplayTask.EndTask` _serverwaittargetdatatask))))