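; Primary-fire gameplay ability for the Tracer minigun that drives automatic fire while input is held.
; It lazily caches the source weapon plus the handle and instance of GA_TracerMinigunPrimaryInstant.
; After a brief delay, longer when sprinting, it batch-RPC activates that instant ability, then calls FireShot every TimeBetweenShot.
; Input release or a failed cost check ends both abilities.
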(event `self.K2_ActivateAbility`
  (`self.CheckAndSetupCachables`
    (:`Is Valid`
      ;[1 1 1] Blend out of running animation
      (if (`GameplayTagAssetInterface.HasMatchingGameplayTag` (`self.GetAbilitySystemComponentFromActorInfo`) (struct :`TagName` "State.Sprinting"))
        (`AbilityTask_WaitDelay.WaitDelay` 0.03
          (:`OnFinish`
            _))
        (else
          ;[1 1 1] One Frame for any montage and stop
          (`AT_WaitDelayOneFrame.WaitDelayOneFrame`
            (:`then`
              _))))
      (bind _returnvalue (`self.BatchRPCTryActivateAbility` (`self.InstantAbilityHandle`)))
      ;[1 1 1] Firemode brances start
      (if _returnvalue
        ;[1 1 1] End both abilities when release
        (`AbilityTask_WaitInputRelease.WaitInputRelease` true
          (:`then`
            ;[1 1 1] Continue to fire shot
            (`AbilityTask_WaitDelay.WaitDelay` (`self.TimeBetweenShot`) :!label _label
              (:`OnFinish`
                (bind _returnvalue_2 (`self.K2_CheckAbilityCost`))
                (if _returnvalue_2
                  (`/Game/Blueprint/Player/Ability/GA_TracerMinigunPrimaryInstant.FireShot` (`self.InstantAbility`))
                  (goto _label)
                  (else
                    _)))))
          (:`OnRelease`
            _))
        (`self.K2_EndAbility` (`self.InstantAbility`))
        (`self.K2_EndAbility`)
        (else
          (`self.K2_EndAbility`))))))