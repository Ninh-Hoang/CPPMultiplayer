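; Gameplay ability that makes the ARTSurvivor player aim toward the cursor while the input is held.
; Activation caches the player and movement component, applies an aiming effect and starts a LookAtCursor task.
; Input release starts a second LookAtCursor task, applies an aiming-removal effect and ends the ability.
; Ending ensures the removal effect has been applied, then removes both effects and stops the tasks.
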(event `self.K2_ActivateAbility`
  (bind (_owneractor _avataractor _playercontroller _abilitysystemcomponent _skeletalmeshcomponent _animinstance _movementcomponent) (break `GameplayAbilityActorInfo` (`self.GetActorInfo`)))
  (set `self.GE_Removal` (struct))
  (`/Engine/EditorBlueprintResources/StandardMacros.IsValid` (`self.Player`)
    (:`Is Valid`
      _)
    (:`Is Not Valid`
      (bind _asartsurvivor (cast `ARTSurvivor` (`self.GetAvatarActorFromActorInfo`)))
      (set `self.Player` _asartsurvivor)))
  (bind _returnvalue (`self.BP_ApplyGameplayEffectToOwner` (`self.GE_Aiming_Class`) 1 (`self.GetAbilityLevel`)))
  (set `self.GE_Aiming` _returnvalue)
  (`/Engine/EditorBlueprintResources/StandardMacros.IsValid` (`self.CharacterMovementComponent`)
    (:`Is Valid`
      _)
    (:`Is Not Valid`
      (bind _ascharacter_movement_component (cast `CharacterMovementComponent` _movementcomponent))
      (set `self.CharacterMovementComponent` _ascharacter_movement_component)))
  (bind _asynctaskproxy (`ATLookAtCursor.LookAtCursor` "None" (`self.Player`) (`self.CharacterMovementComponent`) _playercontroller))
  (set `self.AimTask` _asynctaskproxy)
  (`AbilityTask_WaitInputRelease.WaitInputRelease` true
    (:`OnRelease`
      (bind _asynctaskproxy_2 (`ATLookAtCursor.LookAtCursor` "None" (`self.Player`) (`self.CharacterMovementComponent`) _playercontroller))
      (set `self.AimResetTask` _asynctaskproxy_2)
      (bind _returnvalue_2 (`self.BP_ApplyGameplayEffectToOwner` (`self.GE_AimingRemoval_Class`) (`self.GetAbilityLevel`)))
      (set `self.GE_Removal` _returnvalue_2)
      (`self.K2_EndAbility`))))

(event `self.K2_OnEndAbility`
  (params (bWasCancelled :type Boolean))
  (bind _aimresettask (`self.AimResetTask`))
  (bind _aimtask (`self.AimTask`))
  (bind _returnvalue (`AbilitySystemBlueprintLibrary.GetActiveGameplayEffectStackCount` (`self.GE_Removal`)))
  (if (not (> _returnvalue 0))
    (bind _returnvalue_2 (`self.BP_ApplyGameplayEffectToOwner` (`self.GE_AimingRemoval_Class`) (`self.GetAbilityLevel`)))
    (set `self.GE_Removal` _returnvalue_2))
  (`self.BP_RemoveGameplayEffectFromOwnerWithHandle` (`self.GE_Aiming`))
  (`self.BP_RemoveGameplayEffectFromOwnerWithHandle` (`self.GE_Removal`))
  (`/Engine/EditorBlueprintResources/StandardMacros.IsValid` _aimtask
    (:`Is Valid`
      (`GameplayTask.EndTask` _aimtask)
      (`/Engine/EditorBlueprintResources/StandardMacros.IsValid` _aimresettask
        (:`Is Valid`
          (`GameplayTask.EndTask` _aimresettask))))))