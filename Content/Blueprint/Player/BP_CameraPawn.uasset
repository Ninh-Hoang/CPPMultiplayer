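; Player camera pawn whose graph turns mouse and key input into RTS-style orders for the first selected unit.
; Right-click moves, Q attacks with the Eye shoot tag after an order error check, and R triggers Drifter explode; Shift queues moves and attacks.
; Cursor traces supply order targets and debug spheres.
; E applies a damage GameplayEffect to the selected unit, and an insert-order branch is unwired.
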(event `Key|RightMouseButton`
  (params (Key :type "Key Structure"))
  (bind (_bblockinghit _binitialoverlap _time _distance _location _impactpoint _normal _impactnormal _physmat _hitactor) (`GameplayStatics.BreakHitResult` (`PlayerController.GetHitResultUnderCursorByChannel` (`GameplayStatics.GetPlayerController` 0) "TraceTypeQuery1" true)))
  (:`Pressed`
    (`ARTOrderHelper.IssueOrder` (`|GetArrayItem` (`self.GetSelectedUnit`)) (make `ARTOrderData` "/Game/Blueprint/Order/Or_SimpleMove.Or_SimpleMove_C" true (`KismetMathLibrary.Conv_VectorToVector2D` _location) _hitactor))
    (`KismetSystemLibrary.DrawDebugSphere` _location 30.0 12 (struct :`R` 1.0 :`G` 1.0 :`B` 1.0 :`A` 1.0) 1.0 1.0 :!label _label)))

(event `Key|Shift+RightMouseButton`
  (params (Key :type "Key Structure"))
  (bind (_bblockinghit _binitialoverlap _time _distance _location _impactpoint _normal _impactnormal _physmat _hitactor) (`GameplayStatics.BreakHitResult` (`PlayerController.GetHitResultUnderCursorByChannel` (`GameplayStatics.GetPlayerController` 0) "TraceTypeQuery1" true)))
  (:`Pressed`
    (`ARTOrderHelper.EnqueueOrder` (`|GetArrayItem` (`self.GetSelectedUnit`)) (make `ARTOrderData` "/Game/Blueprint/Order/Or_SimpleMove.Or_SimpleMove_C" true (`KismetMathLibrary.Conv_VectorToVector2D` _location) _hitactor))
    (goto _label)))

(event `Key|Q`
  (params (Key :type "Key Structure"))
  (bind _output (`|GetArrayItem` (`self.GetSelectedUnit`)))
  (bind (_bblockinghit _binitialoverlap _time _distance _location _impactpoint _normal _impactnormal _physmat _hitactor) (`GameplayStatics.BreakHitResult` (`PlayerController.GetHitResultUnderCursorForObjects` (`GameplayStatics.GetPlayerController` 0) (`|MakeArray` "ObjectTypeQuery3" :!type "EObjectTypeQuery Enum") true)))
  (bind _artorderdata (make `ARTOrderData` "/Game/Blueprint/Order/Or_AttackTarget.Or_AttackTarget_C" true (`KismetMathLibrary.Conv_VectorToVector2D` _location) _hitactor -1 (struct :`GameplayTags` (struct :`(TagName` "Ability.AI.Eye.Shoot")))))
  (:`Pressed`
    (if (not (`BlueprintGameplayTagLibrary.HasTag` (`.ErrorTags` (break `ARTOrderErrorTags` (`ARTOrderHelper.CheckOrder` _output _artorderdata))) (struct :`TagName` "Order.Error")))
      (`ARTOrderHelper.IssueOrder` _output _artorderdata)
      (`KismetSystemLibrary.DrawDebugSphere` _location 30.0 12 (struct :`R` 1.0 :`G` 1.0 :`B` 1.0 :`A` 1.0) 1.0 1.0 :!label _label_2))))

(event `Key|Shift+Q`
  (params (Key :type "Key Structure"))
  (bind _output (`|GetArrayItem` (`self.GetSelectedUnit`)))
  (bind (_bblockinghit _binitialoverlap _time _distance _location _impactpoint _normal _impactnormal _physmat _hitactor) (`GameplayStatics.BreakHitResult` (`PlayerController.GetHitResultUnderCursorForObjects` (`GameplayStatics.GetPlayerController` 0) (`|MakeArray` "ObjectTypeQuery3" :!type "EObjectTypeQuery Enum") true)))
  (bind _artorderdata (make `ARTOrderData` "/Game/Blueprint/Order/Or_AttackTarget.Or_AttackTarget_C" true (`KismetMathLibrary.Conv_VectorToVector2D` _location) _hitactor -1 (struct :`GameplayTags` (struct :`(TagName` "Ability.AI.Eye.Shoot")))))
  (:`Pressed`
    (if (not (`BlueprintGameplayTagLibrary.HasTag` (`.ErrorTags` (break `ARTOrderErrorTags` (`ARTOrderHelper.CheckOrder` _output _artorderdata))) (struct :`TagName` "Order.Error")))
      (`ARTOrderHelper.EnqueueOrder` _output _artorderdata)
      (goto _label_2))))

(event `Key|R`
  (params (Key :type "Key Structure"))
  (bind (_bblockinghit _binitialoverlap _time _distance _location _impactpoint _normal _impactnormal _physmat _hitactor) (`GameplayStatics.BreakHitResult` (`PlayerController.GetHitResultUnderCursorForObjects` (`GameplayStatics.GetPlayerController` 0) (`|MakeArray` "ObjectTypeQuery3" :!type "EObjectTypeQuery Enum") true)))
  (:`Pressed`
    (`ARTOrderHelper.IssueOrder` (`|GetArrayItem` (`self.GetSelectedUnit`)) (make `ARTOrderData` "/Game/Blueprint/Order/Or_UseAbility.Or_UseAbility_C" true (`KismetMathLibrary.Conv_VectorToVector2D` _location) _hitactor -1 (struct :`GameplayTags` (struct :`(TagName` "Ability.AI.Drifter.Explode")))))
    (goto _label_2)))

(event `Key|E`
  (params (Key :type "Key Structure"))
  (bind _returnvalue (`AbilitySystemBlueprintLibrary.GetAbilitySystemComponent` (`|GetArrayItem` (`self.GetSelectedUnit`))))
  (:`Pressed`
    (bind _returnvalue_2 (`AbilitySystemBlueprintLibrary.AssignTagSetByCallerMagnitude` (`AbilitySystemComponent.MakeOutgoingSpec` :`self` _returnvalue :`GameplayEffectClass` "/Game/Blueprint/Share/AbilityAndEffectBase/GE_DamageBase.GE_DamageBase_C") (struct :`TagName` "Data.Damage") 2.0))
    (`AbilitySystemComponent.BP_ApplyGameplayEffectSpecToSelf` _returnvalue _returnvalue_2)))

(fn `UserConstructionScript`)