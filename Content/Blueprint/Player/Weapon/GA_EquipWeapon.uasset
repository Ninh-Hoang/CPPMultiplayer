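; GA_EquipWeapon is a gameplay ability that gives a weapon to an RTSurvivor avatar and equips it.
; On activation it casts the avatar to ARTSurvivor, stopping if that fails, and passes WeaponToEquip to the survivor's AddWeaponToEquipment.
; It stores the returned weapon, has the survivor equip it and prints a debug message.
; The graph never calls EndAbility.
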(event `self.K2_ActivateAbility`
  (bind _asartsurvivor (cast `ARTSurvivor` (`self.GetAvatarActorFromActorInfo`)))
  (set `self.OwningPlayer` _asartsurvivor)
  (bind _returnvalue (`ARTSurvivor.AddWeaponToEquipment` (`self.OwningPlayer`) (`self.WeaponToEquip`)))
  (set `self.Weapon` _returnvalue)
  (`self.Equip Weapon`))

(event `Equip Weapon`
  (`ARTSurvivor.EquipWeapon` (`self.OwningPlayer`) (`self.Weapon`))
  (`KismetSystemLibrary.PrintString` "Weapon Changed"))