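; Gameplay ability for the player's axe melee combo, chaining backhand, downward and horizontal attack montages.
; Each montage sends an InputBuffer gameplay event that opens a wait for an input press, which plays the next swing; a press after the third loops back to the first.
; A montage completing or blending out ends the ability.
; The movement component is set to attacking on activation and cleared when the ability ends.
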(event `self.K2_ActivateAbility`
  (`parent.K2_ActivateAbility`)
  (`ARTCharacterMovementComponent.StartAttacking` (`.ARTCharacterMovementComponent` (break `ARTGameplayAbilityActorInfo` (`self.BP_GetARTActorInfo`))))
  (bind (_asynctaskproxy _eventtag) (`AT_PlayMontageMeshWaitForEvent.PlayMontageForMeshAndWaitForEvent` "None" (`self.GetOwningComponentFromActorInfo`) "/Game/CustomAsset/BlockOutCharacter/AxePack/standing_melee_attack_backhand_Montage.standing_melee_attack_backhand_Montage" (struct :`GameplayTags` (struct :`(TagName` "Event.Montage.InputBuffer"))) 1.0 "Combo1" :!label _label)
    (:`OnCompleted`
      (`self.K2_EndAbility` :!label _label_2))
    (:`OnBlendOut`
      (goto _label_2))
    (:`EventReceived`
      (if (== _eventtag (struct :`TagName` "Event.Montage.InputBuffer"))
        (`AbilityTask_WaitInputPress.WaitInputPress` false
          (:`OnPress`
            (bind (_asynctaskproxy_2 _eventtag_2) (`AT_PlayMontageMeshWaitForEvent.PlayMontageForMeshAndWaitForEvent` "None" (`self.GetOwningComponentFromActorInfo`) "/Game/CustomAsset/BlockOutCharacter/AxePack/standing_melee_attack_downward_Montage.standing_melee_attack_downward_Montage" (struct :`GameplayTags` (struct :`(TagName` "Event.Montage.InputBuffer"))) 1.0 "Combo1")
              (:`OnCompleted`
                (`self.K2_EndAbility` :!label _label_3))
              (:`OnBlendOut`
                (goto _label_3))
              (:`EventReceived`
                (if (== _eventtag_2 (struct :`TagName` "Event.Montage.InputBuffer"))
                  (`AbilityTask_WaitInputPress.WaitInputPress` false
                    (:`OnPress`
                      (bind (_asynctaskproxy_3 _eventtag_3) (`AT_PlayMontageMeshWaitForEvent.PlayMontageForMeshAndWaitForEvent` "None" (`self.GetOwningComponentFromActorInfo`) "/Game/CustomAsset/BlockOutCharacter/AxePack/standing_melee_attack_horizontal_Montage.standing_melee_attack_horizontal_Montage" (struct :`GameplayTags` (struct :`(TagName` "Event.Montage.InputBuffer"))) 1.0 "Combo1")
                        (:`OnCompleted`
                          (`self.K2_EndAbility` :!label _label_4))
                        (:`OnBlendOut`
                          (goto _label_4))
                        (:`EventReceived`
                          (if (== _eventtag_3 (struct :`TagName` "Event.Montage.InputBuffer"))
                            (`AbilityTask_WaitInputPress.WaitInputPress` false
                              (:`OnPress`
                                (goto _label)))))))))))))))))

(event `self.K2_OnEndAbility`
  (params (bWasCancelled :type Boolean))
  (`parent.K2_OnEndAbility` bWasCancelled)
  (`ARTCharacterMovementComponent.StopAttacking` (`.ARTCharacterMovementComponent` (break `ARTGameplayAbilityActorInfo` (`self.BP_GetARTActorInfo`)))))