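; Gameplay ability that listens for knockback debuffs on its owner and turns strong hits into a knockback event.
; On activation it waits for gameplay effects applied to self that carry the KnockBack debuff tag, ignoring them while the owner is blocking.
; When the knockback strength in the effect context meets a fixed threshold, it sends Event.Block.Knockback with that context as payload.
; It never ends itself.
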(event `self.K2_ActivateAbility`
  (`parent.K2_ActivateAbility`)
  (bind (_asynctaskproxy _source _spechandle) (`AT_WaitGEAppliedSelf_Local.WaitGameplayEffectAppliedToSelf_Local` (struct) (struct) (make `GameplayTagRequirements` (struct) (struct :`GameplayTags` (struct :`(TagName` "State.WeaponAction.Blocking")))) (make `GameplayTagRequirements` (struct :`GameplayTags` (struct :`(TagName` "Effect.Debuff.KnockBack")))) false null)
    (:`OnApplied`
      (if true
        (bind _returnvalue (`AbilitySystemBlueprintLibrary.GetEffectContext` _spechandle))
        (if (>= (`ARTBlueprintFunctionLibrary.EffectContextGetKnockBackStrength` _returnvalue) 20.0)
          (`self.SendGameplayEvent` (struct :`TagName` "Event.Block.Knockback") (make `GameplayEventData` (struct) null null null null _returnvalue)))))))