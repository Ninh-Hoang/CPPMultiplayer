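; Gameplay ability for the player's axe block, applying a blocking effect and movement state until input is released and any knockback finishes.
; Incoming knockback effects, handled after a server net sync, within the parry window only print a debug string.
; Later frontal hits play a block or stamina-depleted reaction montage with curve-offset root-motion knockback, chosen by strength (top tier unimplemented).
; Hits outside the front cone are forwarded as a gameplay event.
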(event `self.K2_ActivateAbility`
  (bind _returnvalue (`self.GetOwningComponentFromActorInfo`))
  (bind _returnvalue_2 (- (`self.KnockBackTime`) (- (`GameplayStatics.GetTimeSeconds`) (`self.TimeAtKnockbackStart`))))
  (`parent.K2_ActivateAbility`)
  (bind _returnvalue_3 (`self.BP_ApplyGameplayEffectToOwner` "/Game/Blueprint/Player/Weapon/Sword/GE_Blocking.GE_Blocking_C"))
  (set `self.BlockGE` _returnvalue_3)
  (`ARTCharacterMovementComponent.StartBlocking` (`.ARTCharacterMovementComponent` (break `ARTGameplayAbilityActorInfo` (`self.BP_GetARTActorInfo`))))
  (set `self.TimeAtStart` (`GameplayStatics.GetTimeSeconds`))
  (bind (_asynctaskproxy _source _spechandle) (`AT_WaitGEAppliedSelf_Local.WaitGameplayEffectAppliedToSelf_Local` (struct) (struct) (struct) (struct) false null)
    (:`then`
      (`AbilityTask_WaitInputRelease.WaitInputRelease` true
        (:`OnRelease`
          (if (> _returnvalue_2 0.0) :!label _label
            (`AbilityTask_WaitDelay.WaitDelay` _returnvalue_2
              (:`OnFinish`
                (goto _label)))
            (else
              (`self.K2_EndAbility`))))))
    (:`OnApplied`
      (`AbilityTask_NetworkSyncPoint.WaitNetSync` "OnlyServerWait"
        (:`OnSync`
          (if (`BlueprintGameplayTagLibrary.HasTag` (`ARTBlueprintFunctionLibrary.GetAssetTagFromSpec` _spechandle) (struct :`TagName` "Effect.Debuff.KnockBack") true)
            (if (> (- (`GameplayStatics.GetTimeSeconds`) (`self.TimeAtStart`)) (`self.ParryWindow`))
              (bind _returnvalue_4 (`AbilitySystemBlueprintLibrary.GetEffectContext` _spechandle))
              (if (`self.IsEffectCauserInFrontCone` _returnvalue_4)
                (if (> (`ARTCharacterBase.GetStamina` (`self.CharacterPawn`)) 0.0)
                  (bind _returnvalue_5 (`KismetMathLibrary.FCeil` (/ (`ARTBlueprintFunctionLibrary.EffectContextGetKnockBackStrength` _returnvalue_4) 20.0)))
                  (switch `int` _returnvalue_5
                    (:`0`
                      (set `self.Path Offset Curve` (`self.KnockBackCurve0`) :!label _label_2)
                      (set `self.KnockBackTime` 0.5)
                      (`AT_PlayMontageMeshWaitForEvent.PlayMontageForMeshAndWaitForEvent` "None" _returnvalue "/Game/CustomAsset/BlockOutCharacter/AxePack/standing_block_react_large_Montage.standing_block_react_large_Montage" (struct) 1.0 "HitReact"
                        (:`then`
                          (`AbilityTask_ApplyRootMotionMoveToForce.ApplyRootMotionMoveToForce` "None" (`Actor.K2_GetActorLocation` (`self.CharacterPawn`)) (`self.KnockBackTime`) false "MOVE_None" true (`self.Path Offset Curve`) "MaintainLastRootMotionVelocity" :!label _label_3
                            (:`then`
                              (set `self.TimeAtKnockbackStart` (`GameplayStatics.GetTimeSeconds`)))))))
                    (:`1`
                      (goto _label_2))
                    (:`2`
                      (`KismetSystemLibrary.PrintString` "OUT OF RANGE")))
                  (else
                    (switch `int` _returnvalue_5
                      (:`0`
                        (set `self.Path Offset Curve` (`self.KnockBackCurve0`) :!label _label_4)
                        (set `self.KnockBackTime` 0.5)
                        (`AT_PlayMontageMeshWaitForEvent.PlayMontageForMeshAndWaitForEvent` "None" _returnvalue "/Game/CustomAsset/BlockOutCharacter/AxePack/standing_react_large_from_right_Montage.standing_react_large_from_right_Montage"
                          (:`then`
                            (goto _label_3))))
                      (:`1`
                        (goto _label_4))
                      (:`2`
                        (`KismetSystemLibrary.PrintString` "OUT OF RANGE")))))
                (else
                  (`self.SendGameplayEvent` (struct :`TagName` "Event.Block.Knockback") (make `GameplayEventData` (struct) null null null null _returnvalue_4))))
              (else
                (`KismetSystemLibrary.PrintString` "PARY")))))))))

(event `self.K2_OnEndAbility`
  (params (bWasCancelled :type Boolean))
  (`parent.K2_OnEndAbility` bWasCancelled)
  (`self.BP_RemoveGameplayEffectFromOwnerWithHandle` (`self.BlockGE`))
  (`ARTCharacterMovementComponent.StopBlocking` (`.ARTCharacterMovementComponent` (break `ARTGameplayAbilityActorInfo` (`self.BP_GetARTActorInfo`)))))

(fn `IsEffectCauserInFrontCone`
  (params (EffectContext :type "GameplayEffectContextHandle Structure"))
  (returns (ReturnValue :type Boolean))
  (bind _characterpawn (`self.CharacterPawn`))
  (return (<= (`KismetMathLibrary.DegAcos` (`KismetMathLibrary.Dot_VectorVector` (`Actor.GetActorForwardVector` _characterpawn) (`KismetMathLibrary.Normal` (- (`Actor.K2_GetActorLocation` (`AbilitySystemBlueprintLibrary.EffectContextGetEffectCauser` EffectContext)) (`Actor.K2_GetActorLocation` _characterpawn))))) (`self.BlockAngle`))))