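; Gameplay ability for an instant knockback reaction, triggered by a gameplay event.
; It plays a large hit-react montage on the owning mesh and calls StartBlocking on the ART character movement component.
; Completion or blend-out cancels the ability, while interruption or cancellation ends it.
; OnEndAbility calls StopBlocking to release the movement component.
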(event `self.K2_ActivateAbilityFromEvent`
  (params (EventData :type "GameplayEventData Structure (by ref)"))
  (`parent.K2_ActivateAbilityFromEvent` EventData)
  (`AT_PlayMontageMeshWaitForEvent.PlayMontageForMeshAndWaitForEvent` "None" (`self.GetOwningComponentFromActorInfo`) "/Game/CustomAsset/AnimStarterPack/UE4_Mannequin/AxePack/standing_react_large_from_right_Montage.standing_react_large_from_right_Montage"
    (:`then`
      (`ARTCharacterMovementComponent.StartBlocking` (`.ARTCharacterMovementComponent` (break `ARTGameplayAbilityActorInfo` (`self.BP_GetARTActorInfo`)))))
    (:`OnCompleted`
      (`self.K2_CancelAbility` :!label _label))
    (:`OnBlendOut`
      (goto _label))
    (:`OnInterrupted`
      (`self.K2_EndAbility` :!label _label_2))
    (:`OnCancelled`
      (goto _label_2))))

(event `self.K2_OnEndAbility`
  (params (bWasCancelled :type Boolean))
  (`parent.K2_OnEndAbility` bWasCancelled)
  (`ARTCharacterMovementComponent.StopBlocking` (`.ARTCharacterMovementComponent` (break `ARTGameplayAbilityActorInfo` (`self.BP_GetARTActorInfo`)))))