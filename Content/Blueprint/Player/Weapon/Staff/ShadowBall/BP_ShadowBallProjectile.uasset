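; Shadow Ball staff projectile that turns into a lingering damage-and-slow area where it first overlaps anything but its instigator.
; On overlap it stops, enables the AoE sphere, sets a post-hit lifespan and draws a debug sphere.
; The authority applies the effect container to hostile entrants and stores per-actor handles to remove on exit, while remote overlaps destroy the actor.
; The timed re-application and voxel trace are disconnected.
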(event `self.ReceiveBeginPlay`
  ;[1 1 1] Use the local player's ASC since we can't guarantee AI ASC's will still exist if they die after firing
  (bind _asartcharacter_base (cast `ARTCharacterBase` (`self.GetInstigator`)))
  (bind _asartability_system_component (cast `ARTAbilitySystemComponent` (`AbilitySystemBlueprintLibrary.GetAbilitySystemComponent` (`Controller.PlayerState` (`GameplayStatics.GetPlayerController` 0)))))
  (set `self.ASC` _asartability_system_component)
  ;[1 1 1] Muzzle FX will play for locally controlled player on the Instant Ability
  (if (`Pawn.IsLocallyControlled` _asartcharacter_base)
    _))

(event `TickApplyEffect`
  (bind _damageeffectcontainerspec (`self.DamageEffectContainerSpec`))
  ;[1 1 1] Tick apply effect - seem to be quite expensive
  (`ARTBlueprintFunctionLibrary.ClearEffectContainerSpecTargets` _damageeffectcontainerspec)
  (`ARTBlueprintFunctionLibrary.AddTargetsToEffectContainerSpec` :`ContainerSpec` _damageeffectcontainerspec :`TargetActors` (`self.HitTargets`))
  (`ARTBlueprintFunctionLibrary.ApplyExternalEffectContainerSpec` _damageeffectcontainerspec))

(event `self.Sphere.OnComponentBeginOverlap`
  (params (OverlappedComponent :type "PrimitiveComponent Object Reference") (OtherActor :type "Actor Object Reference") (OtherComp :type "PrimitiveComponent Object Reference") (OtherBodyIndex :type Integer) (bFromSweep :type Boolean) (SweepResult :type "HitResult Structure (by ref)"))
  (bind _aoesphere (`self.AoeSphere`))
  (bind _lifetimeafterhit (`self.LifeTimeAfterHit`))
  (if (!= OtherActor (`self.GetInstigator`))
    (`MovementComponent.StopMovementImmediately` (`self.ProjectileMovement`))
    (`PrimitiveComponent.SetCollisionEnabled` (`self.Sphere`) "NoCollision")
    (add `PrimitiveComponent.OnComponentBeginOverlap` _aoesphere (delegate `ResidualAoe`))
    (add `PrimitiveComponent.OnComponentEndOverlap` _aoesphere (delegate `OnLeaveAoE`))
    (`PrimitiveComponent.SetCollisionProfileName` _aoesphere "Aura" true)
    (`PrimitiveComponent.SetCollisionEnabled` _aoesphere "QueryAndPhysics")
    (`self.SetLifeSpan` _lifetimeafterhit)
    (`KismetSystemLibrary.DrawDebugSphere` (`self.K2_GetActorLocation`) 300.0 12 (struct :`R` 1.0 :`G` 1.0 :`B` 1.0 :`A` 1.0) _lifetimeafterhit)))

(event `ResidualAoe`
  (params (OverlappedComponent :type "PrimitiveComponent Object Reference") (OtherActor :type "Actor Object Reference") (OtherComp :type "PrimitiveComponent Object Reference") (OtherBodyIndex :type Integer) (bFromSweep :type Boolean) (SweepResult :type "HitResult Structure (by ref)"))
  (bind _damageeffectcontainerspec (`self.DamageEffectContainerSpec`))
  (`/Engine/EditorBlueprintResources/ActorMacros.Switch Has Authority`
    (:`Authority`
      (bind _returnvalue (`ARTBlueprintFunctionLibrary.MakeTargetDataFromHit` (`GameplayStatics.MakeHitResult` false false 0.0 0.0 (0.0 0.0 0.0) (0.0 0.0 0.0) (0.0 0.0 1.0) (0.0 0.0 1.0) null OtherActor)))
      (bind _returnvalue_2 (`AbilitySystemBlueprintLibrary.FilterTargetData` _returnvalue (`ARTBlueprintFunctionLibrary.MakeTargetDataFilterByTeamAttitude` null (`self.GetInstigator`) "Hostile" "TDFS_Any")))
      (if (`AbilitySystemBlueprintLibrary.TargetDataHasActor` _returnvalue_2)
        (`KismetArrayLibrary.Array_AddUnique` (`self.HitTargets`) OtherActor)
        (`ARTBlueprintFunctionLibrary.ClearEffectContainerSpecTargets` _damageeffectcontainerspec)
        (`ARTBlueprintFunctionLibrary.AddTargetsToEffectContainerSpec` _damageeffectcontainerspec (`|MakeArray` _returnvalue_2))
        (bind _returnvalue_3 (`ARTBlueprintFunctionLibrary.ApplyExternalEffectContainerSpec` _damageeffectcontainerspec))
        (`BlueprintMapLibrary.Map_Add` (`self.Actor/DamageEffectHandle`) OtherActor (`|GetArrayItem` _returnvalue_3))
        (`BlueprintMapLibrary.Map_Add` (`self.Actor/SlowEffectHandle`) OtherActor (`|GetArrayItem` _returnvalue_3 1))))
    (:`Remote`
      (`self.K2_DestroyActor`))))

(event `OnLeaveAoE`
  (params (OverlappedComponent :type "PrimitiveComponent Object Reference") (OtherActor :type "Actor Object Reference") (OtherComp :type "PrimitiveComponent Object Reference") (OtherBodyIndex :type Integer))
  (bind _returnvalue (`AbilitySystemBlueprintLibrary.GetAbilitySystemComponent` OtherActor))
  (bind _hittargets (`self.HitTargets`))
  (`/Engine/EditorBlueprintResources/ActorMacros.Switch Has Authority`
    (:`Authority`
      (if (`KismetArrayLibrary.Array_Contains` _hittargets OtherActor)
        (`AbilitySystemComponent.RemoveActiveGameplayEffect` _returnvalue (`BlueprintMapLibrary.Map_Find` (`self.Actor/DamageEffectHandle`) OtherActor) 1)
        (`AbilitySystemComponent.RemoveActiveGameplayEffect` _returnvalue (`BlueprintMapLibrary.Map_Find` (`self.Actor/SlowEffectHandle`) OtherActor) 1)
        (`KismetArrayLibrary.Array_RemoveItem` _hittargets OtherActor)))
    (:`Remote`
      (`self.K2_DestroyActor`))))

(fn `UserConstructionScript`)