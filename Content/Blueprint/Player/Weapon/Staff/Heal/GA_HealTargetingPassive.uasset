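; Passive staff ability that lets the player target friendly characters and heal them.
; The local player runs the weapon's reusable sphere-trace target actor with a reticle, confirming on input press and handling data on a cast montage event.
; The server handles client target data through a persistent wait task.
; Targets are healed one at a time via RepeatAction, each committing cost and applying a SetByCaller healing effect.
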(event `self.K2_ActivateAbility`
  (`self.CheckAndSetupCachable`)
  (bind (_asynctaskproxy _data) (`AT_ServerWaitForClientTargetData.ServerWaitForClientTargetData` "None")
    (:`then`
      (set `self.ServerWaitTargetData_Task` _asynctaskproxy)
      (`self.StartTargeting`))
    (:`ValidData`
      (`self.HandleTargetData` _data))))

(event `StartTargeting`
  (bind _spheretracetargetactor (`self.SphereTraceTargetActor`))
  ;[1 1 1] Only fire bullets (generate target data) on the local player
  (if (`Controller.IsLocalPlayerController` (`.PlayerController` (break `GameplayAbilityActorInfo` (`self.GetActorInfo`))))
    (set `self.TraceStart` (make `GameplayAbilityTargetingLocationInfo` "SocketTransform" "0.000000,0.000000,0.000000|0.000000,0.000000,0.000000|1.000000,1.000000,1.000000" (`self.CharacterPawn`) (`Equipment.GetEquipmentMesh` (`self.SourceWeapon`)) null "CastSocket"))
    (`GATA_SphereTrace.Configure` :`self` _spheretracetargetactor :`InStartLocation` (`self.TraceStart`) :`InTraceProfile` (struct :`Name` "Projectile") :`InFilter` (`ARTBlueprintFunctionLibrary.MakeTargetDataFilterByTeamAttitude` null (struct) false "Friendly" "TDFS_Any") :`InReticleClass` "/Game/Blueprint/Share/Reticle/BP_SingleTargetReticle.BP_SingleTargetReticle_C" :`bInIgnoreSourceActor` true :`InMaxRange` (`self.MaxRange`) :`InMaxHitResultsPerTrace` (`self.MaxTargets`))
    (bind (_asynctaskproxy _data) (`AT_WaitTargetDataUsingActor.WaitTargetDataWithReusableActor` "HealTarget" "CustomMulti" _spheretracetargetactor true)
      (:`then`
        (set `self.WaitTargetDataWithActor_Task` _asynctaskproxy)
        (`AbilityTask_WaitInputPress.WaitInputPress` false :!label _label
          (:`then`
            (`AbilityTask_WaitInputRelease.WaitInputRelease` false
              (:`OnRelease`
                (`AbilityTask_WaitDelay.WaitDelay` (`self.TimeBetweenHeal`)
                  (:`OnFinish`
                    (goto _label))))))
          (:`OnPress`
            (`self.ConfirmTaskByInstanceName` "HealTarget")
            (bind _returnvalue (`self.K2_CheckAbilityCost`))
            (if _returnvalue
              (`AT_PlayMontageMeshWaitForEvent.PlayMontageForMeshAndWaitForEvent` "None" (`Character.Mesh` (`self.CharacterPawn`)) "/Game/CustomAsset/PolySha/PolySha_Anim_HeavyCast_Montage.PolySha_Anim_HeavyCast_Montage" (struct :`GameplayTags` (struct :`(TagName` "Event.Montage.Shared.SkillUse")))
                (:`EventReceived`
                  (`self.HandleTargetData` (`self.TargetData`))))))))
      (:`ValidData`
        ;[1 1 1] Confirm Target as Button Press in case player aim lose aim
        (set `self.TargetData` _data)))))

(event `HandleTargetData`
  (params (Data :type "GameplayAbilityTargetDataHandle Structure"))
  (bind (_asynctaskproxy _actionnumber) (`AbilityTask_Repeat.RepeatAction` (`self.TimeBetweenHeal`) (`KismetMathLibrary.Min` (`AbilitySystemBlueprintLibrary.GetDataCountFromTargetData` Data) (`self.MaxTargets`)))
    (:`then`
      (set `self.RepeatAction_Task` _asynctaskproxy))
    (:`OnPerformAction`
      (bind _returnvalue (`AbilitySystemBlueprintLibrary.GetHitResultFromTargetData` Data _actionnumber))
      (cast `ARTCharacterBase` (`.HitActor` (`GameplayStatics.BreakHitResult` _returnvalue)))
      (bind _returnvalue_2 (`self.K2_CommitAbilityCost` false))
      (if _returnvalue_2
        (bind _returnvalue_3 (`self.MakeEffectContainerSpec` (struct :`TagName` "Ability")))
        (bind _returnvalue_4 (`AbilitySystemBlueprintLibrary.AssignTagSetByCallerMagnitude` (`|GetArrayItem` (`.TargetGameplayEffectSpecs` (break `ARTGameplayEffectContainerSpec` _returnvalue_3))) (struct :`TagName` "Data.Healing") (`self.AmountOfHeal`)))
        (`self.K2_ApplyGameplayEffectSpecToTarget` _returnvalue_4 (`AbilitySystemBlueprintLibrary.AbilityTargetDataFromHitResult` _returnvalue))))))

(event `self.K2_OnEndAbility`
  (params (bWasCancelled :type Boolean))
  (`GameplayTask.EndTask` (`self.ServerWaitTargetData_Task`)))