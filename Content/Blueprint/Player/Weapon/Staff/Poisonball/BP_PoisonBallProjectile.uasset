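; Poison ball staff projectile that deals area damage through GAS when its sphere overlaps an actor.
; On authority, overlapping a non-instigator triggers a Pawn sphere trace, gathers living characters, applies its damage effect container to filtered target data, then destroys itself.
; Remote copies just destroy themselves on overlap.
; BeginPlay caches the first player's ASC because AI ASCs may not survive firing; the muzzle FX branch and gameplay cue parameters are unused.
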(event `self.ReceiveBeginPlay`
  (bind _asartcharacter_base (cast `ARTCharacterBase` (`self.GetInstigator`)))
  ;[1 1 1] Use the local player's ASC since we can't guarantee AI ASC's will still exist if they die after firing
  (bind _asartability_system_component (cast `ARTAbilitySystemComponent` (`AbilitySystemBlueprintLibrary.GetAbilitySystemComponent` (`Controller.PlayerState` (`GameplayStatics.GetPlayerController` 0)))))
  (set `self.ASC` _asartability_system_component)
  ;[1 1 1] Muzzle FX will play for locally controlled player on the Instant Ability
  (if (`Pawn.IsLocallyControlled` _asartcharacter_base)
    _))

(event `self.Sphere.OnComponentBeginOverlap`
  (params (OverlappedComponent :type "PrimitiveComponent Object Reference") (OtherActor :type "Actor Object Reference") (OtherComp :type "PrimitiveComponent Object Reference") (OtherBodyIndex :type Integer) (bFromSweep :type Boolean) (SweepResult :type "HitResult Structure (by ref)"))
  (bind _returnvalue (`self.K2_GetActorLocation`))
  (bind _damageeffectcontainerspec (`self.DamageEffectContainerSpec`))
  (`/Engine/EditorBlueprintResources/ActorMacros.Switch Has Authority`
    (:`Authority`
      (`KismetSystemLibrary.PrintString` (`KismetTextLibrary.Conv_TextToString` (`|FormatText` "Warning: Rocket Overlap Impacted: {A}" (`KismetTextLibrary.Conv_ObjectToText` null))))
      (if (!= OtherActor (`self.GetInstigator`))
        (bind _outhits (`KismetSystemLibrary.SphereTraceMultiForObjects` _returnvalue (+ _returnvalue 0.01) (`self.Radius`) (`|MakeArray` "ObjectTypeQuery3" :!type "EObjectTypeQuery Enum")))
        (for _array_element _outhits
          (bind _asartcharacter_base (cast `ARTCharacterBase` (`.HitActor` (`GameplayStatics.BreakHitResult` _array_element))))
          (if (`ARTCharacterBase.IsAlive` _asartcharacter_base)
            (`KismetArrayLibrary.Array_AddUnique` (`self.HitTargets`) _asartcharacter_base)))
        (for _array_element_2 (`self.HitTargets`)
          (`KismetArrayLibrary.Array_Add` (`self.HitResult`) (`GameplayStatics.MakeHitResult` false false 0.0 0.0 (0.0 0.0 0.0) (0.0 0.0 0.0) (0.0 0.0 1.0) (0.0 0.0 1.0) null _array_element_2)))
        (bind _returnvalue_2 (`ARTBlueprintFunctionLibrary.MakeArrayTargetDataFromHitArray` (`self.HitResult`)))
        (for _array_element_3 _returnvalue_2
          (`KismetArrayLibrary.Array_Add` (`self.TargetData`) (`AbilitySystemBlueprintLibrary.FilterTargetData` _array_element_3 (`ARTBlueprintFunctionLibrary.MakeTargetDataFilterByActorType` (`|GetArrayItem` (`AbilitySystemBlueprintLibrary.GetActorsFromTargetData` _array_element_3)) (`self.GetOwner`) "Pawns" "TDFS_NoSelf"))))
        (`ARTBlueprintFunctionLibrary.AddTargetsToEffectContainerSpec` _damageeffectcontainerspec (`self.TargetData`))
        (`ARTBlueprintFunctionLibrary.ApplyExternalEffectContainerSpec` _damageeffectcontainerspec)
        (`self.K2_DestroyActor`)))
    (:`Remote`
      (`self.K2_DestroyActor`))))

(fn `UserConstructionScript`)