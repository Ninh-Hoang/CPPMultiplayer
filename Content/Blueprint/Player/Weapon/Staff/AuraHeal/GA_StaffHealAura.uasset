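; Gameplay ability for the staff's healing aura around the wielding character.
; On authority it attaches a sphere component, waits a frame, then sizes it to AuraRadius, enables query collision and adds the aura gameplay cue.
; Friendly actors entering the sphere receive the container's effect, with handles stored per actor.
; On exit that effect is removed and GE_StaffAuraInhibit is applied.
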(event `self.K2_ActivateAbility`
  (bind _spherecollision (`self.SphereCollision`))
  (`self.CheckAndSetupCachables`)
  (if (`Actor.HasAuthority` (`self.CharacterPawn`))
    (bind (_asynctaskproxy _outcomponent) (`AT_SpawnActorComponent.SpawnActorComponent` "/Script/Engine.SphereComponent" "None" (`self.CharacterPawn`))
      (:`OnSuccess`
        (bind _assphere_collision (cast `SphereComponent` _outcomponent))
        (bind _output_get (set `self.SphereCollision` _assphere_collision))
        (`PrimitiveComponent.SetCollisionEnabled` _output_get "NoCollision")
        (add `PrimitiveComponent.OnComponentBeginOverlap` _output_get (delegate `OnAuraStartOverlap`))
        (add `PrimitiveComponent.OnComponentEndOverlap` _output_get (delegate `OnAuraEndOverlap`))
        (`AT_WaitDelayOneFrame.WaitDelayOneFrame`
          (:`OnFinish`
            (`SphereComponent.SetSphereRadius` (`self.SphereCollision`) (`self.AuraRadius`) true)
            (`PrimitiveComponent.SetCollisionProfileName` _spherecollision "Aura" false)
            (`PrimitiveComponent.SetCollisionEnabled` _spherecollision "QueryOnly")
            (`self.K2_AddGameplayCue` (struct :`TagName` "GameplayCue.Ability.Aura.StaffHeal"))))))))

(event `OnAuraStartOverlap`
  (params (OverlappedComponent :type "PrimitiveComponent Object Reference") (OtherActor :type "Actor Object Reference") (OtherComp :type "PrimitiveComponent Object Reference") (OtherBodyIndex :type Integer) (bFromSweep :type Boolean) (SweepResult :type "HitResult Structure (by ref)"))
  (bind _returnvalue (`ARTBlueprintFunctionLibrary.MakeTargetDataFromHit` (`GameplayStatics.MakeHitResult` false false 0.0 0.0 (0.0 0.0 0.0) (0.0 0.0 0.0) (0.0 0.0 1.0) (0.0 0.0 1.0) null OtherActor)))
  (if (`AbilitySystemBlueprintLibrary.TargetDataHasActor` (`AbilitySystemBlueprintLibrary.FilterTargetData` _returnvalue (`ARTBlueprintFunctionLibrary.MakeTargetDataFilterByTeamAttitude` null (`self.CharacterPawn`) "Friendly" "TDFS_Any")))
    (bind _returnvalue_2 (`self.MakeEffectContainerSpec` (struct :`TagName` "Ability")))
    (bind _returnvalue_3 (`self.K2_ApplyGameplayEffectSpecToTarget` (`|GetArrayItem` (`.TargetGameplayEffectSpecs` (break `ARTGameplayEffectContainerSpec` _returnvalue_2))) _returnvalue))
    (`BlueprintMapLibrary.Map_Add` (`self.ActorGameplayEffectMap`) OtherActor (`|GetArrayItem` _returnvalue_3))))

(event `OnAuraEndOverlap`
  (params (OverlappedComponent :type "PrimitiveComponent Object Reference") (OtherActor :type "Actor Object Reference") (OtherComp :type "PrimitiveComponent Object Reference") (OtherBodyIndex :type Integer))
  (bind _returnvalue (`AbilitySystemBlueprintLibrary.GetAbilitySystemComponent` OtherActor))
  (bind _actorgameplayeffectmap (`self.ActorGameplayEffectMap`))
  (if (`BlueprintMapLibrary.Map_Contains` _actorgameplayeffectmap OtherActor)
    (`/Engine/EditorBlueprintResources/StandardMacros.IsValid` _returnvalue
      (:`Is Valid`
        (`AbilitySystemComponent.RemoveActiveGameplayEffect` _returnvalue (`BlueprintMapLibrary.Map_Find` _actorgameplayeffectmap OtherActor) -1)
        (bind _returnvalue_2 (`ARTBlueprintFunctionLibrary.MakeTargetDataFromHit` (`GameplayStatics.MakeHitResult` false false 0.0 0.0 (0.0 0.0 0.0) (0.0 0.0 0.0) (0.0 0.0 1.0) (0.0 0.0 1.0) null OtherActor)))
        (`self.BP_ApplyGameplayEffectToTarget` _returnvalue_2 "/Game/Blueprint/Player/Weapon/Staff/AuraHeal/GE_StaffAuraInhibit.GE_StaffAuraInhibit_C")
        (`BlueprintMapLibrary.Map_Remove` (`self.ActorGameplayEffectMap`) OtherActor)))))