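; Gameplay ability that performs the character's dodge roll.
; On activation it caches the character and movement component, waits briefly when sprinting or one frame otherwise, then checks and commits the ability cost.
; It plays a sped-up dodge montage on the mesh and ends when the montage finishes, blends out or is stopped, or when the cost check fails.
; Logic to turn the character toward last movement input is present but disconnected.
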(event `self.K2_ActivateAbility`
  (`self.SetupCacheable`)
  ;[1 1 1] Wait for blending animation
  (if (`GameplayTagAssetInterface.HasMatchingGameplayTag` (`self.GetAbilitySystemComponentFromActorInfo`) (struct :`TagName` "State.Sprinting"))
    (`AbilityTask_WaitDelay.WaitDelay` 0.03
      (:`then`
        _))
    (else
      ;[1 1 1] Wait one frame for montage to finish
      (`AT_WaitDelayOneFrame.WaitDelayOneFrame`
        (:`then`
          _))))
  (bind _returnvalue (`self.K2_CheckAbilityCost`))
  (if _returnvalue
    (`self.K2_CommitAbilityCost` false)
    (if (`Pawn.IsPlayerControlled` (`self.Character`))
      _
      (else
        _))
    (`AT_PlayMontageMeshWaitForEvent.PlayMontageForMeshAndWaitForEvent` "None" (`Character.Mesh` (`self.Character`)) "/Game/CustomAsset/PolySha/PolySha_Anim_Dodge_Montage.PolySha_Anim_Dodge_Montage" (struct) 1.5
      (:`OnCompleted`
        _)
      (:`OnBlendOut`
        _)
      (:`OnInterrupted`
        _)
      (:`OnCancelled`
        _))
    (`self.K2_EndAbility`)
    (else
      (`self.K2_EndAbility`))))