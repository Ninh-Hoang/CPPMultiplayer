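; GA_Punch3 is a melee punch Gameplay Ability that plays a zombie punching montage on the character mesh.
; Activation caches the character, spawns a target actor, then waits briefly if sprinting or one frame otherwise before checking cost.
; An AttackHit montage event applies set-by-caller damage through an effect container, and AttackEnd ends the ability.
; The montage task listens only for AttackStart, which neither branch handles.
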(event `self.K2_ActivateAbility`
  ;[1 1 1] Blend Animation
  (`self.SetupCachable`)
  (if (`GameplayTagAssetInterface.HasMatchingGameplayTag` (`self.GetAbilitySystemComponentFromActorInfo`) (struct :`TagName` "State.Sprinting"))
    (`AbilityTask_WaitDelay.WaitDelay` 0.1
      (:`OnFinish`
        _))
    (else
      ;[1 1 1] Delay one frame for montage to stop
      (`AT_WaitDelayOneFrame.WaitDelayOneFrame`
        (:`OnFinish`
          _))))
  (bind _returnvalue (`self.K2_CheckAbilityCost`))
  (if _returnvalue
    (bind (_asynctaskproxy _eventtag) (`AT_PlayMontageMeshWaitForEvent.PlayMontageForMeshAndWaitForEvent` "None" (`Character.Mesh` (`self.Character`)) "/Game/CustomAsset/NakedBoiIK/Zombie_Punching_Montage.Zombie_Punching_Montage" (struct :`GameplayTags` (struct :`(TagName` "Event.Montage.AttackStart") :`(TagName` "Event.Montage.AttackEnd") :`(TagName` "Event.Montage.Shared.AttackHit"))) 1.0 "None" false)
      (:`OnCompleted`
        (`self.K2_EndAbility`))
      (:`OnInterrupted`
        (`self.K2_CancelAbility` :!label _label))
      (:`OnCancelled`
        (goto _label))
      (:`EventReceived`
        (if (== _eventtag (struct :`TagName` "Event.Montage.Shared.AttackHit"))
          (`self.HandleData` (struct))
          (elif (== _eventtag (struct :`TagName` "Event.Montage.AttackEnd"))
            (`self.K2_EndAbility`)))))
    (else
      (`self.K2_EndAbility`))))

(event `HandleData`
  (params (Data :type "GameplayAbilityTargetDataHandle Structure"))
  (bind _returnvalue (`self.MakeEffectContainerSpec` (struct :`TagName` "Ability")))
  (bind (_targetdata _targetgameplayeffectspecs) (break `ARTGameplayEffectContainerSpec` _returnvalue))
  (bind _returnvalue_2 (`AbilitySystemBlueprintLibrary.AssignTagSetByCallerMagnitude` (`|GetArrayItem` _targetgameplayeffectspecs) (struct :`TagName` "Data.Damage") (`self.Damage`)))
  (`self.K2_ApplyGameplayEffectSpecToTarget` _returnvalue_2 _targetdata))

(event `self.K2_OnEndAbility`
  (params (bWasCancelled :type Boolean))
  (bind _waittargettask (`self.WaitTargetTask`))
  (`/Engine/EditorBlueprintResources/StandardMacros.IsValid` _waittargettask
    (:`Is Valid`
      (`GameplayTask.EndTask` _waittargettask))))