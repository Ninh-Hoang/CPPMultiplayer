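; Gameplay ability for the TracerHealGun's instant primary shot, applying healing and stun effects to the traced target.
; The local player rate-limits shots against GA_TracerHealGunPrimary and traces from the muzzle with a reusable target actor, while the server waits for replicated target data.
; Both paths feed HandleTargetData, which commits cost, applies the SetByCaller heal and stun, and fires a GameplayCue carrying the hit result.
; PlayFireMontage is an empty stub.
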(event `self.K2_ActivateAbility`
  (`self.CheckAndSetupCachables`)
  (`GATA_Trace.ResetSpread` (`self.LineTraceTargetActor`))
  ;[1 1 1] Tell the Server to start waiting for replicated TargetData. Client simply returns from the Task's Activate(). If the player is the Server (Host), this won't do anything since the TargetData is never RPC'd and the bullet will be handled through the FireBullet event.
  (bind (_asynctaskproxy _data) (`AT_ServerWaitForClientTargetData.ServerWaitForClientTargetData` "None")
    (:`then`
      (set `self.ServerWaitTargetDataTask` _asynctaskproxy)
      (`self.FireShot`))
    (:`ValidData`
      (`self.HandleTargetData` _data))))

(event `FireShot`
  (bind _linetracetargetactor (`self.LineTraceTargetActor`))
  (if (`Controller.IsLocalPlayerController` (`.PlayerController` (break `GameplayAbilityActorInfo` (`self.GetActorInfo`))))
    (if (>= (`KismetMathLibrary.Abs` (- (`GameplayStatics.GetTimeSeconds`) (`self.TimeOfLastShot`))) (- (`/Game/Blueprint/Player/Weapon/TracerHealGun/GA_TracerHealGunPrimary.TimeBetweenShot` (`self.GA_Primary`)) 0.01))
      (bind _returnvalue (`self.K2_CheckAbilityCost`))
      (if _returnvalue
        (`/Engine/EditorBlueprintResources/StandardMacros.IsValid` (`self.SourceWeapon`)
          (:`Is Valid`
            (set `self.TraceStartLocation` (make `GameplayAbilityTargetingLocationInfo` "SocketTransform" "0.000000,0.000000,0.000000|0.000000,0.000000,0.000000|1.000000,1.000000,1.000000" null (`self.WeaponMesh`) null "MuzzleSocket"))
            (set `self.TraceFromPlayerViewPoint` false)
            (set `self.TraceWithPawnOrientation` true)
            (`GATA_LineTrace.Configure` :`self` _linetracetargetactor :`InStartLocation` (`self.TraceStartLocation`) :`InAimingTag` (`self.AimingTag`) :`InAimingRemovalTag` (`self.AimingRemovalTag`) :`InTraceProfile` (struct :`Name` "PhysicsActor") :`bInTraceWithPawnOrientation` (`self.TraceWithPawnOrientation`) :`bInTraceFromPlayerViewPoint` (`self.TraceFromPlayerViewPoint`) :`bInUseAimingSpreadMod` true :`InMaxRange` (`self.TraceRange`) :`InBaseSpread` (`self.WeaponSpread`) :`InAimingSpreadMod` (`self.AimingSpreadMod`) :`InTargetingSpreadIncrement` (`self.FiringSpreadIncreasement`) :`InTargetingSpreadMax` (`self.FiringSpreadMax`))
            (bind (_asynctaskproxy _data) (`AT_WaitTargetDataUsingActor.WaitTargetDataWithReusableActor` "None" "Instant" _linetracetargetactor true)
              (:`then`
                (set `self.TimeOfLastShot` (`GameplayStatics.GetTimeSeconds`)))
              (:`ValidData`
                ;[1 1 1] Handle shot locally - predict hit impact FX or apply damage if player is Host
                (`self.HandleTargetData` _data))))
          (:`Is Not Valid`
            (`KismetSystemLibrary.PrintString` "Source Weapon is Null")))
        (else
          (`self.K2_CancelAbility`)))
      (else
        (`KismetSystemLibrary.PrintString` "Error: Tried to fire a bullet too fast")))))

(event `HandleTargetData`
  (params (Data :type "GameplayAbilityTargetDataHandle Structure"))
  (bind _returnvalue (`self.K2_CommitAbilityCost` false))
  (if _returnvalue
    (`self.PlayFireMontage`)
    (bind _returnvalue_2 (`AbilitySystemBlueprintLibrary.AssignTagSetByCallerMagnitude` (`self.MakeOutgoingGameplayEffectSpec` "/Game/Blueprint/Player/Weapon/TracerHealGun/GE_TracerHealGunHealing.GE_TracerHealGunHealing_C") (struct :`TagName` "Data.Healing") (`self.BulletHeal`)))
    (`self.K2_ApplyGameplayEffectSpecToTarget` _returnvalue_2 Data)
    (`self.BP_ApplyGameplayEffectToTarget` Data "/Game/Blueprint/Player/Weapon/TracerHealGun/GE_TracerHealGun_Stun.GE_TracerHealGun_Stun_C")
    (bind _returnvalue_3 (`AbilitySystemBlueprintLibrary.GetEffectContext` _returnvalue_2))
    (`AbilitySystemBlueprintLibrary.EffectContextAddHitResult` _returnvalue_3 (`AbilitySystemBlueprintLibrary.GetHitResultFromTargetData` Data))
    (`self.K2_ExecuteGameplayCueWithParams` (struct :`TagName` "GameplayCue.Weapon.TracerHealGun.Fire") (`AbilitySystemBlueprintLibrary.MakeGameplayCueParameters` 0.0 0.0 _returnvalue_3))
    (else
      (`self.K2_CancelAbility`))))