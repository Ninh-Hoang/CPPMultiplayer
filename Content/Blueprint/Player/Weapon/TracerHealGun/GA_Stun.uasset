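; GA_Stun is a Gameplay Ability for the TracerHealGun that, despite its name, plays a downward melee attack montage.
; Activation prints a debug message, caches the character and target actor, waits briefly, checks cost, then plays the montage at high rate until end or cancel.
; Melee socket targeting, which would feed GE_SwordMelee damage through HandleData, is disconnected along with the impact cue, so no stun or damage is applied.
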(event `self.K2_ActivateAbility`
  (`KismetSystemLibrary.PrintString` "Hello")
  ;[1 1 1] Blend Animation
  (`self.SetupCachable`)
  (if (`GameplayTagAssetInterface.HasMatchingGameplayTag` (`self.GetAbilitySystemComponentFromActorInfo`) (struct :`TagName` "State.Sprinting"))
    (`AbilityTask_WaitDelay.WaitDelay` 0.0
      (:`then`
        _))
    (else
      ;[1 1 1] Delay one frame for montage to stop
      (`AT_WaitDelayOneFrame.WaitDelayOneFrame`
        (:`then`
          _))))
  (bind _returnvalue (`self.K2_CheckAbilityCost`))
  (if _returnvalue
    (bind (_asynctaskproxy _eventtag) (`AT_PlayMontageMeshWaitForEvent.PlayMontageForMeshAndWaitForEvent` "None" (`Character.Mesh` (`self.Character`)) "/Game/AnimStarterPack/MX_Animation/MT_melee_attack_downward.MT_melee_attack_downward" (struct :`GameplayTags` (struct :`(TagName` "Event.Montage.AttackStart") :`(TagName` "Event.Montage.AttackEnd"))) 4.0)
      (:`OnCompleted`
        (`self.K2_EndAbility` :!label _label))
      (:`OnBlendOut`
        (goto _label))
      (:`OnInterrupted`
        (`self.K2_CancelAbility` :!label _label_2))
      (:`OnCancelled`
        (goto _label_2)))
    (else
      (`self.K2_EndAbility`))))

(event `MeleeDataHandle`
  (`self.ConfirmTaskByInstanceName` "Target"))

(event `HandleData`
  (params (Data :type "GameplayAbilityTargetDataHandle Structure"))
  (bind _returnvalue (`AbilitySystemBlueprintLibrary.AssignTagSetByCallerMagnitude` (`self.MakeOutgoingGameplayEffectSpec` "/Game/Blueprint/Player/Weapon/Sword/GE_SwordMelee.GE_SwordMelee_C") (struct :`TagName` "Data.Damage") (`self.Damage`)))
  (`self.K2_ApplyGameplayEffectSpecToTarget` _returnvalue Data)
  (bind _returnvalue_2 (`AbilitySystemBlueprintLibrary.GetEffectContext` _returnvalue)))

(event `self.K2_OnEndAbility`
  (params (bWasCancelled :type Boolean))
  (bind _waittargettask (`self.WaitTargetTask`))
  (`/Engine/EditorBlueprintResources/StandardMacros.IsValid` _waittargettask
    (:`Is Valid`
      (`GameplayTask.EndTask` _waittargettask))))