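; Gameplay ability for the survivor's hold-to-aim on right mouse button, applying an aiming effect and starting aim-down-sights on the ART movement component.
; It eases the camera along relative X while held and back on release, ending afterward unless a re-press loops back into aiming.
; On end it applies a removal effect, then removes both effects and stops aim-down-sights.
; An alternative LookAtCursor task version remains as unreachable nodes.
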(event `self.K2_ActivateAbility`
  (bind _cameracomponent (`ARTSurvivor.CameraComponent` (`self.Player`)))
  (set `self.GE_Removal` (struct))
  (`/Engine/EditorBlueprintResources/StandardMacros.IsValid` (`self.Player`)
    (:`Is Valid`
      _)
    (:`Is Not Valid`
      (bind _asartsurvivor (cast `ARTSurvivor` (`self.GetAvatarActorFromActorInfo`)))
      (set `self.Player` _asartsurvivor)))
  (bind _returnvalue (`self.BP_ApplyGameplayEffectToOwner` (`self.GE_Aiming_Class`) 1 (`self.GetAbilityLevel`)))
  (set `self.GE_Aiming` _returnvalue)
  (bind _asartcharacter_movement_component (cast `ARTCharacterMovementComponent` (`.MovementComponent` (break `GameplayAbilityActorInfo` (`self.GetActorInfo`)))))
  (`ARTCharacterMovementComponent.StartAimDownSights` _asartcharacter_movement_component)
  (set `self.bCancelAim?` false :!label _label)
  (`AbilityTask_WaitInputRelease.WaitInputRelease` true ; When the player releases Right Mouse Button, end the ability
    (:`then`
      (`KismetSystemLibrary.MoveComponentTo` _cameracomponent (300.0 77.099548 0.0) (struct) true true :!label _label_2))
    (:`OnRelease`
      (`|ExecutionSequence`
        (:`then_0`
          (goto _label_2 :!via `Stop`))
        (:`then_1`
          (`AbilityTask_WaitInputPress.WaitInputPress` true
            (:`then`
              (`KismetSystemLibrary.MoveComponentTo` _cameracomponent (-0.000916 77.099548 0.0) (struct) true true :!label _label_3)
              (if (`self.bCancelAim?`)
                (goto _label)
                (else
                  (`self.K2_EndAbility`))))
            (:`OnPress`
              (set `self.bCancelAim?` true)
              (goto _label_3 :!via `Stop`))))))))

(event `self.K2_OnEndAbility`
  (params (bWasCancelled :type Boolean))
  (bind _returnvalue (`AbilitySystemBlueprintLibrary.GetActiveGameplayEffectStackCount` (`self.GE_Removal`)))
  (if (not (> _returnvalue 0))
    (bind _returnvalue_2 (`self.BP_ApplyGameplayEffectToOwner` (`self.GE_AimingRemoval_Class`) (`self.GetAbilityLevel`)))
    (set `self.GE_Removal` _returnvalue_2))
  (`self.BP_RemoveGameplayEffectFromOwnerWithHandle` (`self.GE_Aiming`))
  (`self.BP_RemoveGameplayEffectFromOwnerWithHandle` (`self.GE_Removal`))
  (bind _asartcharacter_movement_component (cast `ARTCharacterMovementComponent` (`.MovementComponent` (break `GameplayAbilityActorInfo` (`self.GetActorInfo`)))))
  (`ARTCharacterMovementComponent.StopAimDownSights` _asartcharacter_movement_component))