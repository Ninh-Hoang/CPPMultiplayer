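; Gameplay ability for the chainer part of the wand's chain lightning, applying lightning damage to its targets.
; On activation it caches the avatar as a character, waits briefly, then builds an effect container spec from the Ability tag.
; It sets LightningDamage on the first effect spec through SetByCaller Data.Damage, applies that spec to the target data, then applies the whole container and ends.
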(event `self.K2_ActivateAbility`
  (`self.CheckAndSetupCachables`)
  (`AbilityTask_WaitDelay.WaitDelay` 0.1
    (:`OnFinish`
      (bind _returnvalue (`self.MakeEffectContainerSpec` (struct :`TagName` "Ability")))
      (bind (_targetdata _targetgameplayeffectspecs) (break `ARTGameplayEffectContainerSpec` _returnvalue))
      (bind _returnvalue_2 (`AbilitySystemBlueprintLibrary.AssignTagSetByCallerMagnitude` (`|GetArrayItem` _targetgameplayeffectspecs) (struct :`TagName` "Data.Damage") (`self.LightningDamage`)))
      (`self.K2_ApplyGameplayEffectSpecToTarget` _returnvalue_2 _targetdata)
      (`self.ApplyEffectContainerSpec` _returnvalue)
      (`self.K2_EndAbility`))))