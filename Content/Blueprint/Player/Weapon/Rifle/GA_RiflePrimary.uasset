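; Rifle primary-fire gameplay ability that drives automatic fire while the input is held.
; It caches the source weapon and GA_RiflePrimaryInstant instance, then activates that ability through a batched RPC after a short delay for animation transitions.
; A timed loop calls FireBullet on the instant ability every TimeBetweenShot while the cost check passes.
; Input release or a failed cost check ends both abilities.
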(event `self.K2_ActivateAbility`
  (`self.CheckAndSetupCacheables`)
  ;[1 1 1] Blend Animation from gun running to gun shooting
  (if (`GameplayTagAssetInterface.HasMatchingGameplayTag` (`self.GetAbilitySystemComponentFromActorInfo`) (struct :`TagName` "State.Sprinting"))
    (`AbilityTask_WaitDelay.WaitDelay` 0.03
      (:`then`
        _))
    (else
      ;[1 1 1] Delay one frame so montage like reload can stop
      (`AT_WaitDelayOneFrame.WaitDelayOneFrame`
        (:`then`
          _))))
  (bind _returnvalue (`self.BatchRPCTryActivateAbility` (`self.InstantAbilityHandle`)))
  (if _returnvalue
    ;[1 1 1] End Both Ability when release trigger
    (`AbilityTask_WaitInputRelease.WaitInputRelease` true
      (:`then`
        (`AbilityTask_WaitDelay.WaitDelay` (`self.TimeBetweenShot`) :!label _label
          (:`OnFinish`
            (bind _returnvalue_2 (`self.K2_CheckAbilityCost`))
            (if _returnvalue_2
              (`/Game/Blueprint/Player/Weapon/Rifle/GA_RiflePrimaryInstant.FireBullet` (`self.InstantAbility`))
              (goto _label)
              (else
                _)))))
      (:`OnRelease`
        _))
    (`self.K2_EndAbility` (`self.InstantAbility`))
    (`self.K2_EndAbility`)
    (else
      (`self.K2_EndAbility`))))