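; RTS player controller that handles unit selection and group move orders.
; Left mouse press and release tell the HUD to start and stop selection; events clear or add to the selected units.
; Right click creates a new flock through the AI Conductor, registers each selected unit as a boid, then issues AI MoveTo.
; Destinations keep each unit's offset from the group's bounds center, applied to the cursor hit point, preserving formation.
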(event `Key|LeftMouseButton`
  (params (Key :type "Key Structure"))
  (bind _returnvalue (`self.GetHUD`))
  (:`Pressed`
    (message `/Game/Blueprint/UI/Player/DragSelect/SelectionInterface.StartSelection` _returnvalue))
  (:`Released`
    (message `/Game/Blueprint/UI/Player/DragSelect/SelectionInterface.StopSelection` _returnvalue)))

(event `ClearSelectedUnits`
  (`KismetArrayLibrary.Array_Clear` (`self.SelectedUnits`)))

(event `AddSelectedUnit`
  (params (Unit :type "ARTCharacterAI Object Reference (by ref)"))
  (`KismetArrayLibrary.Array_Add` (`self.SelectedUnits`) Unit))

(event `Key|RightMouseButton`
  (params (Key :type "Key Structure"))
  (bind _selectedunits (`self.SelectedUnits`))
  (:`Pressed`
    (bind _center (`GameplayStatics.GetActorArrayBounds` _selectedunits))
    (set `self.CenterOfGroup` _center)
    (set `self.LocationToMove` (`.Location` (`GameplayStatics.BreakHitResult` (`self.GetHitResultUnderCursorByChannel` (`GameplayStatics.GetPlayerController` 0) "TraceTypeQuery1" true))))
    (bind _returnvalue (`ARTAIConductor.CreateFlock` (`ARTGameState.GetAIConductor`)))
    (set `self.CurrentFlock` _returnvalue)
    (for _array_element _selectedunits
      (`ARTAIConductor.TryAddBoidToList` (`ARTGameState.GetAIConductor`) (`self.CurrentFlock`) _array_element))
    (for _array_element_2 _selectedunits
      (`|AIMoveTo` _array_element_2 _array_element_2 (+ (- (`self.K2_GetActorLocation` _array_element_2) (`self.CenterOfGroup`)) (`self.LocationToMove`)) null))))

(fn `UserConstructionScript`)