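; Gameplay ability for a basic shot that applies damage effects to the avatar's ordered target.
; On activation it checks cooldown, then reads the Order_Target actor from the avatar's blackboard.
; It builds an effect container for that actor, sets a fixed Data.Damage set-by-caller magnitude, applies it directly without a projectile, then commits and ends.
; A target-score override favors closer actors when choosing order targets.
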(event `self.K2_ActivateAbility`
  (`parent.K2_ActivateAbility`)
  (bind _returnvalue (`self.K2_CheckAbilityCooldown`))
  (if _returnvalue
    (bind _asactor (cast `Actor` (`BlackboardComponent.GetValueAsObject` (`AIBlueprintHelperLibrary.GetBlackboard` (`self.GetAvatarActorFromActorInfo`)) "Order_Target"))
      (:`then`
        (bind _returnvalue_2 (`self.MakeEffectContainerSpec` (struct :`TagName` "Ability")))
        (`ARTBlueprintFunctionLibrary.AddTargetsToEffectContainerSpec` :`ContainerSpec` _returnvalue_2 :`TargetActors` (`|MakeArray` _asactor))
        (`AbilitySystemBlueprintLibrary.AssignTagSetByCallerMagnitude` (`|GetArrayItem` (`.TargetGameplayEffectSpecs` (break `ARTGameplayEffectContainerSpec` _returnvalue_2))) (struct :`TagName` "Data.Damage") 1.0)
        (`self.ApplyEffectContainerSpec` _returnvalue_2)
        (`self.K2_CommitAbility`)
        (`self.K2_EndAbility`))
      (:`CastFailed`
        (`self.K2_EndAbility`)))
    (else
      (`self.K2_EndAbility`))))

(fn `K2_GetTargetScore`
  (params (OrderedActor :type "Actor Object Reference") (TargetData :type "ARTOrderTargetData Structure (by ref)") (Index :type Integer))
  (returns (ReturnValue :type "Float (double-precision)"))
  (return (+ (* -1 (`Actor.GetDistanceTo` OrderedActor (`.Actor` (break `ARTOrderTargetData` TargetData)))) 100000.0)))