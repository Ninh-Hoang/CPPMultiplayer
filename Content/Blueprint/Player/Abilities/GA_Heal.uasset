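; Gameplay ability that heals the current order target by a fixed amount.
; On activation it checks cooldown and target validity, applies the Ability effect container with a SetByCaller Data.Healing magnitude, then commits and ends.
; The commit happens after the effect is applied, and failed checks just end the ability.
; Target scoring favors actors whose attribute ratio, likely health to max health, is below half, scoring all others zero.
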(event `self.K2_ActivateAbility`
  (bind _returnvalue (`self.GetOrderTarget`))
  (`parent.K2_ActivateAbility`)
  (bind _returnvalue_2 (`self.K2_CheckAbilityCooldown`))
  (if _returnvalue_2
    (`/Engine/EditorBlueprintResources/StandardMacros.IsValid` _returnvalue
      (:`Is Valid`
        (bind _returnvalue_3 (`self.MakeEffectContainerSpec` (struct :`TagName` "Ability")))
        (`ARTBlueprintFunctionLibrary.AddTargetsToEffectContainerSpec` :`ContainerSpec` _returnvalue_3 :`TargetActors` (`|MakeArray` _returnvalue))
        (`AbilitySystemBlueprintLibrary.AssignTagSetByCallerMagnitude` (`|GetArrayItem` (`.TargetGameplayEffectSpecs` (break `ARTGameplayEffectContainerSpec` _returnvalue_3))) (struct :`TagName` "Data.Healing") 200.0)
        (`self.ApplyEffectContainerSpec` _returnvalue_3)
        (`self.K2_CommitAbility`)
        (`self.K2_EndAbility`))
      (:`Is Not Valid`
        (`self.K2_EndAbility`)))
    (else
      (`self.K2_EndAbility`))))

(fn `K2_GetTargetScore`
  (params (OrderedActor :type "Actor Object Reference") (TargetData :type "ARTOrderTargetData Structure (by ref)") (Index :type Integer))
  (returns (ReturnValue :type "Float (double-precision)"))
  (bind _actor (break `ARTOrderTargetData` TargetData))
  (bind (_bsuccessfullyfoundattribute _returnvalue) (`AbilitySystemBlueprintLibrary.GetFloatAttribute` _actor (struct :`AttributeName` "Health" :`Attribute` "/Script/ART.ARTCharacterAttributeSet:Health")))
  (if _bsuccessfullyfoundattribute
    (if (< (/ _returnvalue (`.ReturnValue` (`AbilitySystemBlueprintLibrary.GetFloatAttribute` _actor (struct :`AttributeName` "MaxHealth" :`Attribute` "/Script/ART.ARTCharacterAttributeSet:MaxHealth")))) 0.5)
      (return 100.0)
      (else
        _)))
  (return 0.0))