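; Gameplay ability for a player melee attack that seeks the nearest valid target and motion-warps the avatar toward it.
; A capsule overlap filters pawns by tag requirement and picks the nearest.
; A line trace finds the target's surface, placing the position sync point at an offset from it, capped by warp range.
; With rotation and position warp points set, it plays the montage, ending on completion or without a target.
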(event `self.K2_ActivateAbility`
  (bind _warpcomp (`self.WarpComp`))
  (`parent.K2_ActivateAbility`)
  (`/Engine/EditorBlueprintResources/StandardMacros.IsValid` (`self.WarpComp`)
    (:`Is Valid`
      _)
    (:`Is Not Valid`
      (set `self.WarpComp` (`Actor.GetComponentByClass` (`self.GetAvatarActorFromActorInfo`) "/Script/MotionWarping.MotionWarpingComponent"))))
  (bind _outactor (`self.FindTarget` (`self.SeekRange`)))
  (set `self.SeekingTarget` _outactor)
  (`/Engine/EditorBlueprintResources/StandardMacros.IsValid` (`self.SeekingTarget`)
    (:`Is Valid`
      (`MotionWarpingComponent.AddOrUpdateSyncPoint` _warpcomp "MeleeOneRotation" (make `MotionWarpingSyncPoint` (`Actor.K2_GetActorLocation` (`self.SeekingTarget`)) (struct)))
      (`MotionWarpingComponent.AddOrUpdateSyncPoint` _warpcomp "MeleeOnePosition" (make `MotionWarpingSyncPoint` (`self.FindSyncPoint` (`self.WarpRange`) (`self.OffSetRange`)) (struct)))
      (`AT_PlayMontageMeshWaitForEvent.PlayMontageForMeshAndWaitForEvent` "None" (`self.GetOwningComponentFromActorInfo`) (`self.MontageToPlay`)
        (:`OnCompleted`
          (`self.K2_EndAbility`))))
    (:`Is Not Valid`
      (`self.K2_EndAbility`))))

(fn `FindSyncPoint`
  (params (MaxRange :type "Float (double-precision)") (OffSet :type "Float (double-precision)"))
  (returns (WarpLocation :type "Vector Structure"))
  (locals (Colide :type Boolean) (ImpactPoint :type "Vector Structure" :default (0.0 0.0 0.0)) (OffsetDirection :type "Vector Structure" :default (0.0 0.0 0.0)) (OffsetLocation :type "Vector Structure"))
  (bind _returnvalue (`Actor.K2_GetActorLocation` (`self.GetAvatarActorFromActorInfo`)))
  (bind _returnvalue_2 (`Actor.K2_GetActorLocation` (`self.GetAvatarActorFromActorInfo`)))
  (bind _returnvalue_3 (`KismetMathLibrary.Vector_Distance` _returnvalue_2 (`local.ImpactPoint`)))
  (set `local.OffsetDirection` (`KismetMathLibrary.Normal` (- (`Actor.K2_GetActorLocation` (`self.SeekingTarget`)) _returnvalue)))
  ;[1 1 1] Trace to get actual mesh hit location
  (bind _outhits (`KismetSystemLibrary.LineTraceMultiForObjects` _returnvalue (+ _returnvalue (* (+ (`self.SeekRange`) 500.0) (`local.OffsetDirection`))) (`|MakeArray` "ObjectTypeQuery3" :!type "EObjectTypeQuery Enum")))
  (for _array_element _outhits
    (bind (_bblockinghit _binitialoverlap _time _distance _location _impactpoint _normal _impactnormal _physmat _hitactor) (`GameplayStatics.BreakHitResult` _array_element))
    (if (== (`self.SeekingTarget`) _hitactor)
      (set `local.Colide` true)
      (set `local.ImpactPoint` _impactpoint)
      (break)))
  ;[1 1 1] This should always be true, all in one frame
  (if (`local.Colide`)
    (set `local.OffsetLocation` (+ (`local.ImpactPoint`) (* (* (`local.OffsetDirection`) -1.0) (`local.OffSet`))))
    ;[1 1 1] If warp range + offset < distance to hit, no need to offset
    (if (< _returnvalue_3 (+ (`self.WarpRange`) (`local.OffSet`)))
      ;[1 1 1] If distance to hit < offset, just use current position
      (if (not (< (`KismetMathLibrary.Vector_Distance` (`local.OffsetLocation`) _returnvalue_2) _returnvalue_3))
        (set `local.OffsetLocation` _returnvalue_2))
      (return (`local.OffsetLocation`))
      (else
        (return (+ (`Actor.K2_GetActorLocation` (`self.GetAvatarActorFromActorInfo`)) (* (`local.OffsetDirection`) (`self.WarpRange`))))))
    (else
      (return (`Actor.K2_GetActorLocation` (`self.GetAvatarActorFromActorInfo`))))))

(fn `FindTarget`
  (params (Radius :type "Float (double-precision)"))
  (returns (OutActor :type "Actor Object Reference"))
  (locals (TaggedActors :type "Array of Actor Object Reference"))
  (bind _returnvalue (`Actor.K2_GetActorLocation` (`self.GetAvatarActorFromActorInfo`)))
  (bind (_outactors _returnvalue_2) (`KismetSystemLibrary.CapsuleOverlapActors` _returnvalue Radius 200.0 (`|MakeArray` "ObjectTypeQuery3" :!type "EObjectTypeQuery Enum")))
  (if _returnvalue_2
    (for _array_element _outactors
      (bind _returnvalue_3 (`self.DoesSatisfyTargetTagRequirement` _array_element))
      (if _returnvalue_3
        (`KismetArrayLibrary.Array_Add` (`local.TaggedActors`) _array_element)))
    (return (`.ReturnValue` (`GameplayStatics.FindNearestActor` _returnvalue (`local.TaggedActors`))))
    (else
      (return null))))