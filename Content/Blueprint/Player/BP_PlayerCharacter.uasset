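; Player character Blueprint that seeds a starting inventory and carries test hooks for equipment and damage.
; On BeginPlay, the authority side adds alcohol items and a rifle to the InventoryComponent.
; Hard-wired debug keys equip a tracer rifle with a test print (Z) or call EquipWeapon on the current equipment (C).
; Point damage is only printed to screen, and the construction script is empty.
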(event `self.ReceiveBeginPlay`
  (bind _inventorycomponent (`self.InventoryComponent`))
  (`/Engine/EditorBlueprintResources/ActorMacros.Switch Has Authority`
    (:`Authority`
      (`InventoryComponent.TryAddItemFromClass` _inventorycomponent "/Game/Blueprint/Item/BP_Alcohol_New.BP_Alcohol_New_C" 5)
      (`InventoryComponent.TryAddItemFromClass` _inventorycomponent "/Game/Blueprint/Item/BP_Rifle.BP_Rifle_C" 1))))

(event `Key|Z`
  (params (Key :type "Key Structure"))
  (:`Pressed`
    (`self.EquipItem` "/Game/Blueprint/Weapon/BP_TracerRifle.BP_TracerRifle_C")
    (`KismetSystemLibrary.PrintString` "Hello")))

(event `Key|C`
  (params (Key :type "Key Structure"))
  (:`Pressed`
    (`self.EquipWeapon` (`self.CurrentEquipment`))))

(event `self.ReceivePointDamage`
  (params (Damage :type "Float (single-precision)") (DamageType :type "DamageType Object Reference") (HitLocation :type "Vector Structure") (HitNormal :type "Vector Structure") (HitComponent :type "PrimitiveComponent Object Reference") (BoneName :type Name) (ShotFromDirection :type "Vector Structure") (InstigatedBy :type "Controller Object Reference") (DamageCauser :type "Actor Object Reference") (HitInfo :type "HitResult Structure (by ref)"))
  (`KismetSystemLibrary.PrintString` (`KismetStringLibrary.Conv_DoubleToString` Damage)))

(fn `UserConstructionScript`)