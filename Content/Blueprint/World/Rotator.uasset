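; Rotator is a world actor that continuously spins four of its mesh components.
; On Tick, it multiplies RotationSpeed by delta time and applies the result as frame-rate-independent local rotation.
; StaticMesh1 turns on roll and pitch, StaticMesh on pitch and yaw, while the two GameJamEdgeDamage meshes pitch in opposite directions.
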(event `self.ReceiveTick`
  (params (DeltaSeconds :type "Float (single-precision)"))
  (bind _calrot (`self.CalRot`))
  (bind _calrot_2 (`self.CalRot`))
  (set `self.CalRot` (* DeltaSeconds (`self.RotationSpeed`)))
  (`SceneComponent.K2_AddLocalRotation` (`self.StaticMesh1`) (`KismetMathLibrary.MakeRotator` _calrot _calrot) false false)
  (`SceneComponent.K2_AddLocalRotation` (`self.StaticMesh`) (`KismetMathLibrary.MakeRotator` 0.0 _calrot_2 _calrot_2) false false)
  (`SceneComponent.K2_AddLocalRotation` (`self.GameJam_Edge_Damage_2250_3_0_main_geo`) (`KismetMathLibrary.MakeRotator` 0.0 (`self.CalRot`)) false false)
  (`SceneComponent.K2_AddLocalRotation` (`self.GameJam_Edge_Damage_2250_3_0_main_geo1`) (`KismetMathLibrary.MakeRotator` 0.0 (* (`self.CalRot`) -1.0)) false false))

(fn `UserConstructionScript`)