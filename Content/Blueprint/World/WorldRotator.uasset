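; WorldRotator is an actor that continuously spins three mesh components in the world.
; Each Tick scales RotationSpeed by DeltaSeconds for a frame-rate independent step, then applies it as local rotation.
; StaticMesh tumbles on all three axes, while the two GameJamEdgeDamage geometry components spin on pitch in opposite directions.
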(event `self.ReceiveTick`
  (params (DeltaSeconds :type "Float (single-precision)"))
  (bind _caledrot (`self.CaledRot`))
  (set `self.CaledRot` (* DeltaSeconds (`self.RotationSpeed`)))
  (`SceneComponent.K2_AddLocalRotation` (`self.StaticMesh`) (`KismetMathLibrary.MakeRotator` _caledrot _caledrot _caledrot) false false)
  (`SceneComponent.K2_AddLocalRotation` (`self.GameJam_Edge_Damage_2250_3_0_main_geo`) (`KismetMathLibrary.MakeRotator` 0.0 (`self.CaledRot`)) false false)
  (`SceneComponent.K2_AddLocalRotation` (`self.GameJam_Edge_Damage_2250_3_0_main_geo1`) (`KismetMathLibrary.MakeRotator` 0.0 (* (`self.CaledRot`) -1.0)) false false))

(fn `UserConstructionScript`)