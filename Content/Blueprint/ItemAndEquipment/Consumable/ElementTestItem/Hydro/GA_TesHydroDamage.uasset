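; Test gameplay ability for a Hydro element consumable item that applies an effect container with water damage data.
; On activation it builds the spec from the Ability container tag, sets Data.Damage.Water to zero magnitude on the first target spec, applies it and ends immediately.
; An unconnected branch would link a GE_EleWater effect spec before applying, but it never runs.
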(event `self.K2_ActivateAbility`
  (`parent.K2_ActivateAbility`)
  (bind _returnvalue (`self.MakeEffectContainerSpec` (struct :`TagName` "Ability")))
  (`AbilitySystemBlueprintLibrary.AssignTagSetByCallerMagnitude` (`|GetArrayItem` (`.TargetGameplayEffectSpecs` (break `ARTGameplayEffectContainerSpec` _returnvalue))) (struct :`TagName` "Data.Damage.Water"))
  (`self.ApplyEffectContainerSpec` _returnvalue)
  (`self.K2_EndAbility`))