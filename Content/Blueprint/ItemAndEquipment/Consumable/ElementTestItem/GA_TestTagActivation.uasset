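; Test gameplay ability, named for tag activation, that prints a debug message and plays the owning character pawn's Knockback montage.
; ActivateAbility waits on the montage task, ending the ability on completion or blend out and cancelling it on interruption or cancellation.
; Unwired alternatives remain in the graph: a mesh-specific montage task and a root motion jump force, neither of which runs.
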(event `self.K2_ActivateAbility`
  (`parent.K2_ActivateAbility`)
  (`KismetSystemLibrary.PrintString` "Hello")
  (`AbilityTask_PlayMontageAndWait.CreatePlayMontageAndWaitProxy` "None" (`ARTCharacterBase.Knockback` (`self.CharacterPawn`))
    (:`OnCompleted`
      (`self.K2_EndAbility` :!label _label))
    (:`OnBlendOut`
      (goto _label))
    (:`OnInterrupted`
      (`self.K2_CancelAbility` :!label _label_2))
    (:`OnCancelled`
      (goto _label_2))))