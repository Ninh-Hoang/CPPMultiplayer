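; GA_Knockback is a gameplay ability that plays the character pawn's knockback reaction montage.
; On activation it runs the parent logic, then plays the pawn's Knockback montage on its mesh through a montage-and-wait-for-event task.
; Completion or blend-out ends the ability, while interruption or cancellation cancels it.
; It applies no movement or effects in this graph, and the end-ability override is disabled.
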(event `self.K2_ActivateAbility`
  (bind _characterpawn (`self.CharacterPawn`))
  (`parent.K2_ActivateAbility`)
  (`AT_PlayMontageMeshWaitForEvent.PlayMontageForMeshAndWaitForEvent` "None" (`Character.Mesh` _characterpawn) (`ARTCharacterBase.Knockback` _characterpawn)
    (:`OnCompleted`
      (`self.K2_EndAbility` :!label _label))
    (:`OnBlendOut`
      (goto _label))
    (:`OnInterrupted`
      (`self.K2_CancelAbility` :!label _label_2))
    (:`OnCancelled`
      (goto _label_2))))