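; GA_TestActivation is a test Gameplay Ability, filed among consumable element test items, that is activated by a gameplay event.
; On activation it calls the parent logic, then plays the PolySha dodge montage on the character pawn's mesh.
; When the montage completes, blends out, is interrupted or is cancelled, it ends the ability and prints the event's tag and magnitude for debugging.
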(event `self.K2_ActivateAbilityFromEvent`
  (params (EventData :type "GameplayEventData Structure (by ref)"))
  (bind (_eventtag _instigator _target _optionalobject _optionalobject2 _contexthandle _instigatortags _targettags _eventmagnitude) (break `GameplayEventData` EventData))
  (`parent.K2_ActivateAbilityFromEvent` EventData)
  (`AT_PlayMontageMeshWaitForEvent.PlayMontageForMeshAndWaitForEvent` "None" (`Character.Mesh` (`self.CharacterPawn`)) "/Game/CustomAsset/PolySha/PolySha_Anim_Dodge_Montage.PolySha_Anim_Dodge_Montage"
    (:`OnCompleted`
      _)
    (:`OnBlendOut`
      _)
    (:`OnInterrupted`
      _)
    (:`OnCancelled`
      _))
  (`self.K2_EndAbility`)
  (`KismetSystemLibrary.PrintString` (`KismetStringLibrary.Concat_StrStr` (`KismetStringLibrary.Conv_NameToString` (`BlueprintGameplayTagLibrary.GetTagName` _eventtag)) (`KismetStringLibrary.Conv_DoubleToString` _eventmagnitude))))