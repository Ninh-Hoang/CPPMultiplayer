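; Test gameplay ability, apparently an element test item, that tries to trigger abilities on a targeted character by gameplay tag.
; On activation it commits, builds an effect container spec for its target data, and casts the first hit actor to ARTCharacterBase.
; It calls TryActivateAbilitiesByTag on that character's ability system with remote activation allowed, prints the result, and ends.
; Water damage effect application remains in the graph but never runs.
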(event `self.K2_ActivateAbility`
  (`parent.K2_ActivateAbility`)
  (`self.K2_CommitAbility`)
  (bind _returnvalue (`self.MakeEffectContainerSpec` (struct :`TagName` "Ability")))
  (bind (_bblockinghit _binitialoverlap _time _distance _location _impactpoint _normal _impactnormal _physmat _hitactor) (`GameplayStatics.BreakHitResult` (`AbilitySystemBlueprintLibrary.GetHitResultFromTargetData` (`.TargetData` (break `ARTGameplayEffectContainerSpec` _returnvalue)))))
  (bind _asartcharacter_base (cast `ARTCharacterBase` _hitactor)
    (:`then`
      (`KismetSystemLibrary.PrintString` (`KismetSystemLibrary.GetDisplayName` _hitactor))
      (bind _returnvalue_2 (`AbilitySystemComponent.TryActivateAbilitiesByTag` (`AbilitySystemBlueprintLibrary.GetAbilitySystemComponent` _asartcharacter_base) (`self.NewVar_0`) true))
      (if _returnvalue_2
        (`KismetSystemLibrary.PrintString` "Activate")
        (else
          (`KismetSystemLibrary.PrintString` "Fail")))
      (`self.K2_EndAbility`))
    (:`CastFailed`
      (`self.K2_EndAbility`))))