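; GA_Frozen is an event-activated gameplay ability that freezes a character, part of the Cryo element test item.
; On activation it applies GE_Frozen to its own ASC with prediction, then waits for a both-sides net sync.
; It then slows the current montage on the character mesh to a near standstill and restores normal play rate after a short delay.
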(event `self.K2_ActivateAbilityFromEvent`
  (params (EventData :type "GameplayEventData Structure (by ref)"))
  (bind _asc (`self.ASC`))
  (bind _mesh (`Character.Mesh` (`self.CharacterPawn`)))
  (`parent.K2_ActivateAbilityFromEvent` EventData)
  (`ARTAbilitySystemComponent.BP_ApplyGameplayEffectToSelfWithPrediction` :`self` _asc :`GameplayEffectClass` "/Game/Blueprint/ItemAndEquipment/Consumable/ElementTestItem/Cryo/GE_Frozen.GE_Frozen_C")
  (`AbilityTask_NetworkSyncPoint.WaitNetSync` "BothWait"
    (:`OnSync`
      (`ARTAbilitySystemComponent.BP_SetPlayRateForCurrentMontage` _asc _mesh 0.0001)
      (`AbilityTask_WaitDelay.WaitDelay` 2.0
        (:`OnFinish`
          (`ARTAbilitySystemComponent.BP_SetPlayRateForCurrentMontage` _asc _mesh 1.0))))))

(event `self.K2_OnEndAbility`
  (params (bWasCancelled :type Boolean))
  (`parent.K2_OnEndAbility` bWasCancelled))