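; Gameplay ability for an elemental test consumable that deals electric damage through the Gameplay Ability System.
; On activation it builds an effect container spec from the Ability tag and sets the SetByCaller electric damage magnitude on its first target spec.
; It links a GE_EleElectro spec carrying the same magnitude to that spec, then applies the container and ends immediately.
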(event `self.K2_ActivateAbility`
  (`parent.K2_ActivateAbility`)
  (bind _returnvalue (`self.MakeEffectContainerSpec` (struct :`TagName` "Ability")))
  (bind _output (`|GetArrayItem` (`.TargetGameplayEffectSpecs` (break `ARTGameplayEffectContainerSpec` _returnvalue))))
  (`AbilitySystemBlueprintLibrary.AssignTagSetByCallerMagnitude` _output (struct :`TagName` "Data.Damage.Elec") 1.0)
  (bind _returnvalue_2 (`AbilitySystemBlueprintLibrary.AssignTagSetByCallerMagnitude` (`self.MakeOutgoingGameplayEffectSpec` "/Game/Blueprint/ItemAndEquipment/Consumable/ElementTestItem/GE_EleElectro.GE_EleElectro_C") (struct :`TagName` "Data.Damage.Elec") 1.0))
  (`AbilitySystemBlueprintLibrary.AddLinkedGameplayEffectSpec` _output _returnvalue_2)
  (`self.ApplyEffectContainerSpec` _returnvalue)
  (`self.K2_EndAbility`))