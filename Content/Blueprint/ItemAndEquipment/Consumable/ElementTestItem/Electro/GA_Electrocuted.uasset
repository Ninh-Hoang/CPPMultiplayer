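; Gameplay ability for the electrocuted reaction, activated from a gameplay event, that knocks the character back.
; After calling the parent activation, it plays the character pawn's Knockback montage on its mesh.
; As the montage starts, it removes active effects granting the State.Element.Elec tag.
; The ability ends when the montage completes or blends out, and cancels if it is interrupted or cancelled.
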(event `self.K2_ActivateAbilityFromEvent`
  (params (EventData :type "GameplayEventData Structure (by ref)"))
  (bind _characterpawn (`self.CharacterPawn`))
  (`parent.K2_ActivateAbilityFromEvent` EventData)
  (`AT_PlayMontageMeshWaitForEvent.PlayMontageForMeshAndWaitForEvent` "None" (`Character.Mesh` _characterpawn) (`ARTCharacterBase.Knockback` _characterpawn)
    (:`then`
      (`AbilitySystemComponent.RemoveActiveEffectsWithGrantedTags` (`self.ASC`) (struct :`GameplayTags` (struct :`(TagName` "State.Element.Elec") :`(TagName` "State.Element.Water")))))
    (:`OnCompleted`
      (`self.K2_EndAbility` :!label _label))
    (:`OnBlendOut`
      (goto _label))
    (:`OnInterrupted`
      (`self.K2_CancelAbility` :!label _label_2))
    (:`OnCancelled`
      (goto _label_2))))