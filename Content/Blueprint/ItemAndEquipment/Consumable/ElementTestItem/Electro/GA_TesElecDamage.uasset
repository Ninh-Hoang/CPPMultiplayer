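; Gameplay ability for an Electro element test consumable that applies an effect container through GAS.
; On activation it builds the Ability-tagged container spec, sets its first effect's Data.Damage.Elec SetByCaller magnitude to zero, applies it, then commits and ends.
; Ending also stops any valid gameplay-event wait task.
; A branch linking GE_EleElectro as an additional effect is disconnected, as are other direct effect-application nodes.
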(event `self.K2_ActivateAbility`
  (`parent.K2_ActivateAbility`)
  (bind _returnvalue (`self.MakeEffectContainerSpec` (struct :`TagName` "Ability")))
  (`AbilitySystemBlueprintLibrary.AssignTagSetByCallerMagnitude` (`|GetArrayItem` (`.TargetGameplayEffectSpecs` (break `ARTGameplayEffectContainerSpec` _returnvalue))) (struct :`TagName` "Data.Damage.Elec"))
  (`self.ApplyEffectContainerSpec` _returnvalue)
  (`self.K2_CommitAbility`)
  (`self.K2_EndAbility`))

(event `self.K2_OnEndAbility`
  (params (bWasCancelled :type Boolean))
  (bind _waitgameplayevent_task (`self.WaitGameplayEvent_Task`))
  (`parent.K2_OnEndAbility` bWasCancelled)
  (`/Engine/EditorBlueprintResources/StandardMacros.IsValid` _waitgameplayevent_task
    (:`Is Valid`
      (`GameplayTask.EndTask` _waitgameplayevent_task))))