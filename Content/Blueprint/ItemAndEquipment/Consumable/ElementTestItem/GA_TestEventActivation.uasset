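; Test gameplay ability, activated by a gameplay event, that plays the character's Knockback montage on its mesh.
; As the montage starts it also applies a root motion jump force with negligible distance, keeping the last root motion velocity on finish.
; The ability ends on jump finish, landing, or montage blend-out or completion, and cancels if the montage is interrupted or cancelled.
; A debug sphere at the event's hit location is left unwired.
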(event `self.K2_ActivateAbilityFromEvent`
  (params (EventData :type "GameplayEventData Structure (by ref)"))
  (bind _characterpawn (`self.CharacterPawn`))
  (`parent.K2_ActivateAbilityFromEvent` EventData)
  (`AT_PlayMontageMeshWaitForEvent.PlayMontageForMeshAndWaitForEvent` "None" (`Character.Mesh` _characterpawn) (`ARTCharacterBase.Knockback` _characterpawn) (struct) 1.0 "None" false
    (:`then`
      (`AbilityTask_ApplyRootMotionJumpForce.ApplyRootMotionJumpForce` "None" (struct) 0.02 0.0 0.0 0.0 false "MaintainLastRootMotionVelocity"
        (:`OnFinish`
          _)
        (:`OnLanded`
          _))
      (`self.K2_EndAbility` :!label _label))
    (:`OnCompleted`
      (goto _label))
    (:`OnBlendOut`
      (goto _label))
    (:`OnInterrupted`
      (`self.K2_CancelAbility` :!label _label_2))
    (:`OnCancelled`
      (goto _label_2))))