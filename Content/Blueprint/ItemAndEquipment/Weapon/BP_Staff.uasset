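; BP_Staff is a staff weapon item that a character equips on use.
; OnUse runs only with server authority: the first use adds BP_Staff to the character's equipment and caches the returned weapon, then every use calls EquipWeapon on it.
; An unconnected, unused chain would instead equip through the GA_EquipWeapon gameplay ability, and it references BP_Sword rather than the staff.
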(event `self.OnUse`
  (params (Character :type "ARTSurvivor Object Reference"))
  ;[1 1 1] Only Server call this
  (if (`Actor.HasAuthority` Character)
    (`/Engine/EditorBlueprintResources/StandardMacros.IsValid` (`self.Weapon`)
      (:`Is Valid`
        _)
      (:`Is Not Valid`
        (bind _returnvalue (`ARTSurvivor.AddWeaponToEquipment` Character "/Game/Blueprint/Player/Weapon/Staff/BP_Staff.BP_Staff_C"))
        (set `self.Weapon` _returnvalue)))
    (`ARTSurvivor.EquipWeapon` Character (`self.Weapon`))))