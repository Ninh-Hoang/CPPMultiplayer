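; BP_Sword is a usable sword item that equips its weapon on the character who uses it.
; On use, it adds itself by class to the character's equipment if no valid weapon is cached, stores the result, then tells the character to equip it.
; An unconnected alternative path through the GA_EquipWeapon gameplay ability remains in the graph but never runs.
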(event `self.OnUse`
  (params (Character :type "ARTSurvivor Object Reference"))
  ;[1 1 1] Working Weapon Changing on Server
  (`/Engine/EditorBlueprintResources/StandardMacros.IsValid` (`self.Weapon`)
    (:`Is Valid`
      _)
    (:`Is Not Valid`
      (bind _returnvalue (`ARTSurvivor.AddWeaponToEquipment` Character "/Game/Blueprint/Player/Weapon/Sword/BP_Sword.BP_Sword_C"))
      (set `self.Weapon` _returnvalue)))
  (`ARTSurvivor.EquipWeapon` Character (`self.Weapon`)))