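; Stalker AI gameplay ability that fires a barrage of electric-damage missiles from the body socket.
; Activation requires the blackboard Target to be within range and inside a cone along the socket's forward axis.
; It lowers the turret anim blend rate, draws a debug aim line and builds a SetByCaller effect container.
; After a delay, the authority repeatedly spawns projectiles with random cone spread, passing them that container; ending raises the blend rate.
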(event `self.K2_ActivateAbility`
  (bind _returnvalue (`self.GetAvatarActorFromActorInfo`))
  (bind _returnvalue_2 (`SceneComponent.GetSocketTransform` (`Character.Mesh` (`self.CharacterPawn`)) "bodySocket" "RTS_World"))
  (bind _returnvalue_3 (`KismetMathLibrary.TransformDirection` _returnvalue_2 (1.0 0.0 0.0)))
  (bind _location (.location _returnvalue_2))
  (`parent.K2_ActivateAbility`)
  (bind _asstalker_anim (cast `/Game/Blueprint/AI/Stalker/Stalker_Anim` (`SkeletalMeshComponent.GetAnimInstance` (`Character.Mesh` (`self.CharacterPawn`)))))
  (set `/Game/Blueprint/AI/Stalker/Stalker_Anim.TurrentBlendRate` 1.0 _asstalker_anim)
  (`KismetSystemLibrary.DrawDebugLine` _location (+ _location (* _returnvalue_3 2000.0)) (struct) 2.0 2.0)
  (bind _returnvalue_4 (`self.MakeEffectContainerSpec` (struct :`TagName` "Ability")))
  (`AbilitySystemBlueprintLibrary.AssignTagSetByCallerMagnitude` (`|GetArrayItem` (`.TargetGameplayEffectSpecs` (break `ARTGameplayEffectContainerSpec` _returnvalue_4))) (struct :`TagName` "Data.Damage.Elec") 2.0)
  (set `self.EffectContainer` _returnvalue_4)
  (`AbilityTask_WaitDelay.WaitDelay` 2.0
    (:`OnFinish`
      (if (`Actor.HasAuthority` _returnvalue)
        (`AbilityTask_Repeat.RepeatAction` 0.1 (`self.NumberOfMissles`)
          (:`OnPerformAction`
            (`|SpawnActorFromClass` "/Game/Blueprint/AI/Stalker/Ability/MissleBarrage_Projectile.MissleBarrage_Projectile_C" (`KismetMathLibrary.MakeTransform` _location (`KismetMathLibrary.Conv_VectorToRotator` (`KismetMathLibrary.RandomUnitVectorInConeInRadiansFromStream` _returnvalue_3 (`KismetMathLibrary.DegreesToRadians` (/ (`self.Spread`) 2.0)) (`KismetMathLibrary.MakeRandomStream` (`KismetMathLibrary.RandomInteger` 100))))) "Undefined" "OverrideRootScale" _returnvalue (`self.EffectContainer`) (`self.CharacterPawn`)))
          (:`OnFinished`
            (`self.K2_EndAbility`)))
        (else
          (`self.K2_EndAbility`))))))

(event `self.K2_OnEndAbility`
  (params (bWasCancelled :type Boolean))
  (`parent.K2_OnEndAbility` bWasCancelled)
  (bind _asstalker_anim (cast `/Game/Blueprint/AI/Stalker/Stalker_Anim` (`SkeletalMeshComponent.GetAnimInstance` (`Character.Mesh` (`self.CharacterPawn`)))))
  (set `/Game/Blueprint/AI/Stalker/Stalker_Anim.TurrentBlendRate` 5.0 _asstalker_anim))

(fn `K2_CanActivateAbility`
  (params (ActorInfo :type "GameplayAbilityActorInfo Structure"))
  (returns (RelevantTags :type "GameplayTagContainer Structure") (ReturnValue :type Boolean))
  (locals (InRange :type Boolean) (InCone :type Boolean) (Cone :type "Float (double-precision)" :default 7.0) (Range :type "Float (double-precision)" :default 2200.0))
  (bind (_owneractor _avataractor) (break `GameplayAbilityActorInfo` ActorInfo))
  (bind _returnvalue (`AIBlueprintHelperLibrary.GetBlackboard` _avataractor))
  (bind _returnvalue_2 (`BlackboardComponent.GetValueAsObject` _returnvalue "Target"))
  (`/Engine/EditorBlueprintResources/StandardMacros.IsValid` _returnvalue
    (:`Is Valid`
      (`/Engine/EditorBlueprintResources/StandardMacros.IsValid` _returnvalue_2
        (:`Is Valid`
          (bind _asartcharacter_ai (cast `ARTCharacterAI` _avataractor))
          (bind _asactor (cast `Actor` _returnvalue_2))
          (bind _returnvalue_3 (`SceneComponent.GetSocketTransform` (`Character.Mesh` _asartcharacter_ai) "bodySocket" "RTS_World"))
          (bind _returnvalue_4 (`Actor.K2_GetActorLocation` _asactor))
          (bind _location (.location _returnvalue_3))
          (set `local.InCone` (<= (`KismetMathLibrary.DegAcos` (`KismetMathLibrary.Dot_VectorVector` (`KismetMathLibrary.TransformDirection` _returnvalue_3 (1.0 0.0 0.0)) (`KismetMathLibrary.Normal` (- _returnvalue_4 _location)))) (`local.Cone`)))
          (set `local.InRange` (<= (`KismetMathLibrary.Vector_Distance` _returnvalue_4 _location) (`local.Range`)))
          (if (and (`local.InRange`) (`local.InCone`))
            (return (struct) true)
            (else
              (return (struct) false))))
        (:`Is Not Valid`
          _)))
    (:`Is Not Valid`
      _))
  (return (struct) false))