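; BP_Ranger_Enemy is the Blueprint for a Ranger AI enemy that reacts to damage, threats and cover.
; Point damage draws a debug sphere and the damage number at the hit location, with no damage handling in this graph.
; Threaten sets the IsThreaten Blackboard key when the IsThreaten variable is false, without setting that variable here.
; EnterCover flags the enemy as in cover and crouches it.
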(event `self.ReceivePointDamage`
  (params (Damage :type "Float (single-precision)") (DamageType :type "DamageType Object Reference") (HitLocation :type "Vector Structure") (HitNormal :type "Vector Structure") (HitComponent :type "PrimitiveComponent Object Reference") (BoneName :type Name) (ShotFromDirection :type "Vector Structure") (InstigatedBy :type "Controller Object Reference") (DamageCauser :type "Actor Object Reference") (HitInfo :type "HitResult Structure (by ref)"))
  ;[1 1 1] Draw Debug on Damaged
  (`KismetSystemLibrary.DrawDebugSphere` HitLocation 5.0 12 (struct :`R` 1.0 :`G` 0.087291 :`A` 1.0) 1.0 1.0)
  (`KismetSystemLibrary.DrawDebugString` HitLocation (`KismetStringLibrary.Conv_DoubleToString` Damage) null (struct :`R` 1.0 :`B` 0.018721 :`A` 1.0) 1.0))

(event `self.Threaten`
  (if (not (`self.IsThreaten`))
    (`BlackboardComponent.SetValueAsBool` (`AIBlueprintHelperLibrary.GetBlackboard` null) "IsThreaten" true)))

(event `Enter Cover`
  (set `self.IsInCover` true)
  (`self.Crouch`))

(fn `UserConstructionScript`)