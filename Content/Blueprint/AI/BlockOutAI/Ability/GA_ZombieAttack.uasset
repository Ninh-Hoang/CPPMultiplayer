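; Gameplay ability for the zombie AI's attack, which plays the attack montage on the owner's mesh.
; On the montage's hit event it builds an effect container, setting set-by-caller damage on the first spec and knockback strength on the second's context, then applies it.
; Montage completion or blend-out ends the ability, while interruption cancels it.
; A fixed utility score is returned for ability scoring.
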(event `self.K2_ActivateAbility`
  (`parent.K2_ActivateAbility`)
  (bind (_asynctaskproxy _eventtag _eventdata) (`AT_PlayMontageMeshWaitForEvent.PlayMontageForMeshAndWaitForEvent` "None" (`self.GetOwningComponentFromActorInfo`) "/Game/CustomAsset/BlockOutCharacter/ZombiePack/zombie_attack_Montage.zombie_attack_Montage" (struct :`GameplayTags` (struct :`(TagName` "Event.Montage.Shared.AttackHit"))))
    (:`OnCompleted`
      (`self.K2_EndAbility` :!label _label))
    (:`OnBlendOut`
      (goto _label))
    (:`OnInterrupted`
      (`self.K2_CancelAbility` :!label _label_2))
    (:`OnCancelled`
      (goto _label_2))
    (:`EventReceived`
      (bind _returnvalue (`self.MakeEffectContainerSpec` (struct :`TagName` "Ability") _eventdata))
      (bind (_targetdata _targetgameplayeffectspecs) (break `ARTGameplayEffectContainerSpec` _returnvalue))
      (`AbilitySystemBlueprintLibrary.AssignTagSetByCallerMagnitude` (`|GetArrayItem` _targetgameplayeffectspecs) (struct :`TagName` "Data.Damage") 1.0)
      (bind _returnvalue_2 (`AbilitySystemBlueprintLibrary.GetEffectContext` (`|GetArrayItem` _targetgameplayeffectspecs 1)))
      (`ARTBlueprintFunctionLibrary.EffectContextSetKnockBackStrength` _returnvalue_2 20.0)
      (`self.ApplyEffectContainerSpec` _returnvalue))))

(fn `K2_ScoreAbilityUtility`
  (params (ActorInfo :type "GameplayAbilityActorInfo Structure"))
  (returns (ReturnValue :type "Float (double-precision)"))
  (return 50.0))