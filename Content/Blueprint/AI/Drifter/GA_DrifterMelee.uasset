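; Gameplay ability for the Drifter's melee attack, which plays a montage and deals damage.
; After a minimal delay that varies with the sprinting tag, it checks cost, plays the montage and ends or cancels with it.
; Montage events build effect container specs and apply the first with SetByCaller damage.
; A separate HandleData event applies GE_SwordMelee to supplied target data; the impact cue is unwired.
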(event `self.K2_ActivateAbility`
  ;[1 1 1] Blend Animation
  (`self.SetupCachable`)
  (if (`GameplayTagAssetInterface.HasMatchingGameplayTag` (`self.GetAbilitySystemComponentFromActorInfo`) (struct :`TagName` "State.Sprinting"))
    (`AbilityTask_WaitDelay.WaitDelay` 0.0
      (:`then`
        _))
    (else
      ;[1 1 1] Delay one frame for montage to stop
      (`AT_WaitDelayOneFrame.WaitDelayOneFrame`
        (:`then`
          _))))
  (bind _returnvalue (`self.K2_CheckAbilityCost`))
  (if _returnvalue
    (bind (_asynctaskproxy _eventtag _eventdata) (`AT_PlayMontageMeshWaitForEvent.PlayMontageForMeshAndWaitForEvent` "None" (`Character.Mesh` (`self.Character`)) "/Game/CustomAsset/DrifterProto/DrifterProto_Melee_Montage.DrifterProto_Melee_Montage" (struct :`GameplayTags` (struct :`(TagName` "Event.Montage"))))
      (:`OnCompleted`
        (`self.K2_EndAbility` :!label _label))
      (:`OnBlendOut`
        (goto _label))
      (:`OnInterrupted`
        (`self.K2_CancelAbility` :!label _label_2))
      (:`OnCancelled`
        (goto _label_2))
      (:`EventReceived`
        (bind _returnvalue_2 (`self.MakeEffectContainerSpec` _eventtag _eventdata))
        (bind (_targetdata _targetgameplayeffectspecs) (break `ARTGameplayEffectContainerSpec` _returnvalue_2))
        (bind _returnvalue_3 (`AbilitySystemBlueprintLibrary.AssignTagSetByCallerMagnitude` (`|GetArrayItem` _targetgameplayeffectspecs) (struct :`TagName` "Data.Damage") (`self.Damage`)))
        (`self.K2_ApplyGameplayEffectSpecToTarget` _returnvalue_3 _targetdata)))
    (else
      (`self.K2_EndAbility`))))

(event `HandleData`
  (params (Data :type "GameplayAbilityTargetDataHandle Structure"))
  (bind _returnvalue (`AbilitySystemBlueprintLibrary.AssignTagSetByCallerMagnitude` (`self.MakeOutgoingGameplayEffectSpec` "/Game/Blueprint/Player/Ability/Sword/GE_SwordMelee.GE_SwordMelee_C") (struct :`TagName` "Data.Damage") (`self.Damage`)))
  (`self.K2_ApplyGameplayEffectSpecToTarget` _returnvalue Data)
  (bind _returnvalue_2 (`AbilitySystemBlueprintLibrary.GetEffectContext` _returnvalue)))

(event `self.K2_OnEndAbility`
  (params (bWasCancelled :type Boolean))
  (bind _waittargettask (`self.WaitTargetTask`))
  (`/Engine/EditorBlueprintResources/StandardMacros.IsValid` _waittargettask
    (:`Is Valid`
      (`GameplayTask.EndTask` _waittargettask))))