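; Gameplay ability that fires one hitscan turret shot, using client-predicted target data.
; On activation the server awaits client target data, while the local controller checks fire interval and cost, then traces from the muzzle through a reusable spread-aware LineTrace target actor.
; Both paths feed HandleTargetData, which commits cost, applies SetByCaller rifle damage and executes the fire GameplayCue with the hit result.
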(event `self.K2_ActivateAbility`
  (`self.CheckAndSetupCacheable`
    (:`Is Valid`
      ;[1 1 1] Reset Spread to 0
      (`GATA_Trace.ResetSpread` (`self.LineTraceTargetActor`))
      ;[1 1 1] Tell the Server to start waiting for replicated TargetData. Client simply returns from the Task's Activate(). If the player is the Server (Host), this won't do anything since the TargetData is never RPC'd and the bullet will be handled through the FireBullet event.
      (bind (_asynctaskproxy _data) (`AT_ServerWaitForClientTargetData.ServerWaitForClientTargetData` "None")
        (:`then`
          (set `self.ServerWaitTargetDataTask` _asynctaskproxy)
          (`self.FireBullet`))
        (:`ValidData`
          (`self.HandleTargetData` _data))))))

(event `FireBullet`
  (bind _linetracetargetactor (`self.LineTraceTargetActor`))
  ;[1 1 1] Only (fire) Generate Target Data on local player
  (if (`Controller.IsLocalPlayerController` (`.PlayerController` (break `GameplayAbilityActorInfo` (`self.GetActorInfo`))))
    (if (>= (`KismetMathLibrary.Abs` (- (`GameplayStatics.GetTimeSeconds`) (`self.TimeOfLastShot`))) (- (`/Game/Blueprint/AI/Turret/GA_Turret_Shoot.TimeBetweenShot` (`self.GA_Primary`)) 0.01))
      (bind _returnvalue (`self.K2_CheckAbilityCost`))
      (if _returnvalue
        (set `self.TraceStartLocation` (make `GameplayAbilityTargetingLocationInfo` "LiteralTransform" (`KismetMathLibrary.Conv_VectorToTransform` (`SceneComponent.GetSocketLocation` (`Character.Mesh` (`self.TurretCharacter`)) "MuzzleSocket"))))
        (set `self.TraceWithPawnOrientation` true)
        (set `self.TraceFromPlayerViewpoint` false)
        (`GATA_LineTrace.Configure` :`self` _linetracetargetactor :`InStartLocation` (`self.TraceStartLocation`) :`InAimingTag` (`self.AimingTag`) :`InAimingRemovalTag` (`self.AimingRemovalTag`) :`InTraceProfile` (struct :`Name` "PhysicsActor") :`bInDebug` true :`bInTraceWithPawnOrientation` (`self.TraceWithPawnOrientation`) :`bInTraceFromPlayerViewPoint` (`self.TraceFromPlayerViewpoint`) :`bInUseAimingSpreadMod` true :`InMaxRange` (`self.TraceRange`) :`InBaseSpread` (`self.WeaponSpread`) :`InAimingSpreadMod` (`self.AimingSpreadMod`) :`InTargetingSpreadIncrement` (`self.FiringSpreadIncreasement`) :`InTargetingSpreadMax` (`self.FiringSpreadMax`))
        (bind (_asynctaskproxy _data) (`AT_WaitTargetDataUsingActor.WaitTargetDataWithReusableActor` "None" "Instant" _linetracetargetactor true)
          (:`then`
            (set `self.TimeOfLastShot` (`GameplayStatics.GetTimeSeconds`)))
          (:`ValidData`
            ;[1 1 1] Handle Shot Locally, predict FX or Apply Damage on Server
            (`self.HandleTargetData` _data)))
        (else
          (`self.K2_CancelAbility`)))
      (else
        (`KismetSystemLibrary.PrintString` "Error: Try to Firebullet too fast")))))

(event `HandleTargetData`
  (params (Data :type "GameplayAbilityTargetDataHandle Structure"))
  (bind _returnvalue (`self.K2_CommitAbilityCost` false))
  (if _returnvalue
    (`self.PlayFireMontage`)
    (bind _returnvalue_2 (`AbilitySystemBlueprintLibrary.AssignTagSetByCallerMagnitude` (`self.MakeOutgoingGameplayEffectSpec` "/Game/Blueprint/Player/Ability/Rifle/GE_RifleDamage.GE_RifleDamage_C") (struct :`TagName` "Data.Damage") (`self.BulletDamage`)))
    (`self.K2_ApplyGameplayEffectSpecToTarget` _returnvalue_2 Data)
    (bind _returnvalue_3 (`AbilitySystemBlueprintLibrary.GetEffectContext` _returnvalue_2))
    (`AbilitySystemBlueprintLibrary.EffectContextAddHitResult` _returnvalue_3 (`AbilitySystemBlueprintLibrary.GetHitResultFromTargetData` Data))
    (`self.K2_ExecuteGameplayCueWithParams` (struct :`TagName` "GameplayCue.Weapon.Rifle.Fire") (`AbilitySystemBlueprintLibrary.MakeGameplayCueParameters` 0.0 0.0 _returnvalue_3))
    (else
      (`self.K2_CancelAbility`))))

(event `self.K2_OnEndAbility`
  (params (bWasCancelled :type Boolean))
  (bind _serverwaittargetdatatask (`self.ServerWaitTargetDataTask`))
  (`/Engine/EditorBlueprintResources/StandardMacros.IsValid` _serverwaittargetdatatask
    (:`Is Valid`
      (`GameplayTask.EndTask` _serverwaittargetdatatask))))