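; Gameplay ability for the LegBot AI that handles a part break by stunning the bot.
; On event activation it applies GE_Stun to its owner, passing the Duration variable as a SetByCaller magnitude.
; It then disables collision on the BP_LegBot capsule and ends immediately, without restoring collision itself.
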(event `self.K2_ActivateAbilityFromEvent`
  (params (EventData :type "GameplayEventData Structure (by ref)"))
  (`parent.K2_ActivateAbilityFromEvent` EventData)
  (bind _returnvalue (`AbilitySystemBlueprintLibrary.AssignTagSetByCallerMagnitude` (`self.MakeOutgoingGameplayEffectSpec` "/Game/Blueprint/Share/Effect/Stun/GE_Stun.GE_Stun_C") (struct :`TagName` "Data.GameplayEffect.Duration") (`self.Duration`)))
  (`self.K2_ApplyGameplayEffectSpecToOwner` _returnvalue)
  (bind _asbp_leg_bot (cast `/Game/Blueprint/AI/LegBot/BP_LegBot` (`self.CharacterPawn`)))
  (`PrimitiveComponent.SetCollisionEnabled` (`/Game/Blueprint/AI/LegBot/BP_LegBot.Capsule` _asbp_leg_bot) "NoCollision")
  (`self.K2_EndAbility`))