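; Gameplay ability for the LegBot's twin-gun burst, holding a shooting effect from activation until the ability ends.
; After a delay, it repeats line traces from both gun sockets at a fire-rate interval over a set duration, randomly spreading endpoints within a forward cone.
; Each trace applies set-by-caller electric damage to hostile targets via a team-attitude filter and fires a rifle gameplay cue carrying the hit result.
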(event `self.K2_ActivateAbility`
  (bind _object_types (`self.Object Types`))
  (bind _characterpawn (`self.CharacterPawn`))
  (bind _mesh (`Character.Mesh` _characterpawn))
  (bind _returnvalue (+ (`Actor.K2_GetActorLocation` _characterpawn) (* (`KismetMathLibrary.RandomUnitVectorInConeInRadiansFromStream` (`SceneComponent.GetForwardVector` (`Character.CapsuleComponent` _characterpawn)) (`KismetMathLibrary.DegreesToRadians` (/ (`self.Spread`) 2.0)) (`KismetMathLibrary.MakeRandomStream` (`KismetMathLibrary.RandomInteger` 100))) (`self.Range`))))
  (`parent.K2_ActivateAbility`)
  (bind _returnvalue_2 (`self.K2_CheckAbilityCooldown`))
  (if _returnvalue_2
    (`self.K2_CommitAbility`)
    (bind _returnvalue_3 (`self.BP_ApplyGameplayEffectToOwner` "/Game/Blueprint/AI/LegBot/Ability/GE_LegBot_Shooting.GE_LegBot_Shooting_C"))
    (set `self.GEShootHandle` _returnvalue_3)
    (`AbilityTask_WaitDelay.WaitDelay` (`self.DelayTime`)
      (:`OnFinish`
        (`AbilityTask_Repeat.RepeatAction` (`self.FireRate`) (`KismetMathLibrary.FTrunc` (/ (`self.Duration`) (`self.FireRate`)))
          (:`OnPerformAction`
            (bind _outhit (`KismetSystemLibrary.LineTraceSingleForObjects` (`SceneComponent.GetSocketLocation` _mesh "gunR_Socket") _returnvalue _object_types false (`|MakeArray` _characterpawn :!type "Actor Object Reference") "None" true (struct :`R` 1.0 :`A` 1.0) (struct :`G` 1.0 :`A` 1.0) 2.0))
            (`self.HandleHitResult` _outhit)
            (bind _outhit_2 (`KismetSystemLibrary.LineTraceSingleForObjects` :`Start` (`SceneComponent.GetSocketLocation` _mesh "gunL_Socket") :`End` _returnvalue :`ObjectTypes` _object_types :`DrawTime` 2.0))
            (`self.HandleHitResult` _outhit_2))
          (:`OnFinished`
            (`self.K2_EndAbility`)))))
    (else
      (`self.K2_EndAbility`))))

(event `HandleHitResult`
  (params (Hit :type "HitResult Structure"))
  (bind _returnvalue (`ARTBlueprintFunctionLibrary.MakeTargetDataFromHit` Hit))
  (bind _returnvalue_2 (`AbilitySystemBlueprintLibrary.AssignTagSetByCallerMagnitude` (`self.MakeOutgoingGameplayEffectSpec` "/Game/Blueprint/ItemAndEquipment/Consumable/ElementTestItem/Electro/GE_ElectroDamage.GE_ElectroDamage_C") (struct :`TagName` "Data.Damage.Elec") 0.5))
  (`self.K2_ApplyGameplayEffectSpecToTarget` _returnvalue_2 (`AbilitySystemBlueprintLibrary.FilterTargetData` _returnvalue (`ARTBlueprintFunctionLibrary.MakeTargetDataFilterByTeamAttitude` null (`self.CharacterPawn`) "Hostile" "TDFS_NoSelf")))
  (bind _returnvalue_3 (`AbilitySystemBlueprintLibrary.GetEffectContext` _returnvalue_2))
  (`AbilitySystemBlueprintLibrary.EffectContextAddHitResult` _returnvalue_3 Hit)
  (`self.K2_ExecuteGameplayCueWithParams` (struct :`TagName` "GameplayCue.RifleFire") (`AbilitySystemBlueprintLibrary.MakeGameplayCueParameters` 0.0 0.0 _returnvalue_3)))

(event `self.K2_OnEndAbility`
  (params (bWasCancelled :type Boolean))
  (`parent.K2_OnEndAbility` bWasCancelled)
  (`self.BP_RemoveGameplayEffectFromOwnerWithHandle` (`self.GEShootHandle`)))