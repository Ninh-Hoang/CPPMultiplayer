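; Gameplay ability that teleports the Eye AI character to a location chosen by an EQS query.
; On activation it caches the avatar pawn, runs EQS_FindTeleLocation for a random pick from the best 25%, and plays the teleport montage.
; The montage's SkillUse event triggers a MoveToLocation task to the first query result.
; Montage completion or blend-out ends the ability, while interruption or cancellation cancels it.
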(event `self.K2_ActivateAbility`
  (`self.CheckAndSetupCacheable`)
  (bind _returnvalue (`EnvQueryManager.RunEQSQuery` "/Game/Blueprint/AI/Eye/TelePort/EQS_FindTeleLocation.EQS_FindTeleLocation" (`self.CharacterPawn`) "RandomBest25Pct"))
  (`AT_PlayMontageMeshWaitForEvent.PlayMontageForMeshAndWaitForEvent` "None" (`Character.Mesh` (`self.CharacterPawn`)) "/Game/CustomAsset/Eye/Eye_Anim_Teleport_Montage.Eye_Anim_Teleport_Montage" (struct :`GameplayTags` (struct :`(TagName` "Event.Montage.Shared.SkillUse")))
    (:`OnCompleted`
      (`self.K2_EndAbility` :!label _label))
    (:`OnBlendOut`
      (goto _label))
    (:`OnInterrupted`
      (`self.K2_CancelAbility` :!label _label_2))
    (:`OnCancelled`
      (goto _label_2))
    (:`EventReceived`
      (bind _resultlocations (`EnvQueryInstanceBlueprintWrapper.GetQueryResultsAsLocations` _returnvalue))
      (bind _asynctaskproxy (`AbilityTask_MoveToLocation.MoveToLocation` "None" (`|GetArrayItem` _resultlocations))
        (:`OnTargetLocationReached`
          (`GameplayTask.EndTask` _asynctaskproxy))))))