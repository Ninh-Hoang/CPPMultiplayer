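; Projectile for the Eye AI that applies a gameplay effect container to hostile actors it hits.
; On sphere overlap, the server ignores the instigator and filters hit target data by team attitude against the owner.
; A hostile hit feeds the target into the effect spec, applies it and destroys the projectile, while remote copies destroy themselves on any overlap.
; BeginPlay caches the owner's ability system component.
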(event `self.ReceiveBeginPlay`
  (bind _asartcharacter_base (cast `ARTCharacterBase` (`self.GetInstigator`)))
  ;[1 1 1] Use the local player's ASC since we can't guarantee AI ASC's will still exist if they die after firing
  (bind _asartability_system_component (cast `ARTAbilitySystemComponent` (`AbilitySystemBlueprintLibrary.GetAbilitySystemComponent` (`self.GetOwner`))))
  (set `self.ASC` _asartability_system_component)
  ;[1 1 1] Muzzle FX will play for locally controlled player on the Instant Ability
  (if (`Pawn.IsLocallyControlled` _asartcharacter_base)
    _))

(event `self.Sphere.OnComponentBeginOverlap`
  (params (OverlappedComponent :type "PrimitiveComponent Object Reference") (OtherActor :type "Actor Object Reference") (OtherComp :type "PrimitiveComponent Object Reference") (OtherBodyIndex :type Integer) (bFromSweep :type Boolean) (SweepResult :type "HitResult Structure (by ref)"))
  (bind _gespechandle (`self.GESpecHandle`))
  (`/Engine/EditorBlueprintResources/ActorMacros.Switch Has Authority`
    (:`Authority`
      (if (!= OtherActor (`self.GetInstigator`))
        (bind _returnvalue (`ARTBlueprintFunctionLibrary.MakeTargetDataFromHit` SweepResult))
        (bind _returnvalue_2 (`AbilitySystemBlueprintLibrary.FilterTargetData` _returnvalue (`ARTBlueprintFunctionLibrary.MakeTargetDataFilterByTeamAttitude` OtherActor (`self.GetOwner`) "Hostile" "TDFS_Any")))
        (if (`AbilitySystemBlueprintLibrary.TargetDataHasActor` _returnvalue_2)
          (`ARTBlueprintFunctionLibrary.AddTargetsToEffectContainerSpec` _gespechandle (`|MakeArray` _returnvalue_2))
          (`ARTBlueprintFunctionLibrary.ApplyExternalEffectContainerSpec` _gespechandle)
          (`self.K2_DestroyActor`))))
    (:`Remote`
      (`self.K2_DestroyActor`))))

(fn `UserConstructionScript`)