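; Gameplay ability for the Eye AI's Slow Burst, which applies the ability's effect container and then ends.
; On activation it caches the avatar as an ARTCharacterBase, then builds and immediately applies the container spec under the Ability tag.
; A half-second delay task then ends the ability, with no cleanup logic on end.
; Targeting and the effects themselves come from the container, outside this graph.
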(event `self.K2_ActivateAbility`
  (`self.CheckAndSetupCacheable`)
  (bind _returnvalue (`self.MakeEffectContainerSpec` (struct :`TagName` "Ability")))
  (`self.ApplyEffectContainerSpec` _returnvalue)
  (`AbilityTask_WaitDelay.WaitDelay` 0.5
    (:`OnFinish`
      (`self.K2_EndAbility`))))

(event `self.K2_OnEndAbility`
  (params (bWasCancelled :type Boolean)))