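; RTS HUD that draws a marquee selection box and passes the units inside it to the player controller.
; StartSelection anchors the box at the viewport-scaled mouse position.
; While dragging, DrawHUD renders a translucent rectangle to the cursor and gathers ARTCharacterBase actors inside it each frame.
; StopSelection clears the controller's current selection and adds the gathered actors, cast to ARTCharacterAI.
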(event `self.ReceiveBeginPlay`
  (bind _asbp_wdplayer_controller (cast `/Game/Blueprint/BP_WDPlayerController` (`GameplayStatics.GetPlayerController` 0)))
  (set `self.Controller` _asbp_wdplayer_controller))

(event `/Game/Blueprint/SelectionInterface.StartSelection`
  (bind _returnvalue (`WidgetLayoutLibrary.GetViewportScale`))
  (bind _returnvalue_2 (`WidgetLayoutLibrary.GetMousePositionOnViewport`))
  (bind (_returnvalue_x _returnvalue_y) (`KismetMathLibrary.BreakVector2D` (* _returnvalue_2 (`KismetMathLibrary.MakeVector2D` _returnvalue _returnvalue))))
  (set `self.PointA` (`KismetMathLibrary.MakeVector2D` _returnvalue_x _returnvalue_y))
  (set `self.IsDrawing` true))

(event `/Game/Blueprint/SelectionInterface.StopSelection`
  (set `self.IsDrawing` false)
  (if (`self.IsMarquee`)
    (`/Engine/EditorBlueprintResources/StandardMacros.IsValid` (`self.Controller`)
      (:`Is Valid`
        (`/Game/Blueprint/BP_WDPlayerController.ClearSelectedUnits` (`self.Controller`))
        (for _array_element (`self.SelectionUnits`)
          (bind _asartcharacter_ai (cast `ARTCharacterAI` _array_element))
          (`/Game/Blueprint/BP_WDPlayerController.AddSelectedUnit` (`self.Controller`) _asartcharacter_ai)))
      (:`Is Not Valid`
        _))
    (set `self.IsMarquee` false)))

(event `self.ReceiveDrawHUD`
  (params (SizeX :type Integer) (SizeY :type Integer))
  (bind _returnvalue (`WidgetLayoutLibrary.GetViewportScale`))
  (bind (_pointa_x _pointa_y) (`KismetMathLibrary.BreakVector2D` (`self.PointA`)))
  (bind (_pointb_x _pointb_y) (`KismetMathLibrary.BreakVector2D` (`self.PointB`)))
  (if (`self.IsDrawing`)
    (bind _returnvalue_2 (`WidgetLayoutLibrary.GetMousePositionOnViewport`))
    (bind (_returnvalue_x _returnvalue_y) (`KismetMathLibrary.BreakVector2D` (* _returnvalue_2 (`KismetMathLibrary.MakeVector2D` _returnvalue _returnvalue))))
    (set `self.PointB` (`KismetMathLibrary.MakeVector2D` _returnvalue_x _returnvalue_y))
    (set `self.IsMarquee` true)
    (`self.DrawRect` (struct :`G` 1.0 :`B` 0.880262 :`A` 0.2) _pointa_x _pointa_y (- _pointb_x _pointa_x) (- _pointb_y _pointa_y))
    (set `self.SelectionUnits` (`self.GetActorsInSelectionRectangle` "/Script/ART.ARTCharacterBase" (`self.PointA`) (`self.PointB`)))))

(fn `UserConstructionScript`)