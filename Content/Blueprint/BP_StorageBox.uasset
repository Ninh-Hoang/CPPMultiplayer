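; BP_StorageBox is an interactable storage container that holds items in an Inventory component, initialized in the construction script.
; On interaction it creates a WBP_StorageInventory widget for the interacting character's BasePlayerController, passes itself as the Storage reference, adds it to the viewport and shows the mouse cursor.
; An unconnected debug loop that prints item names is left in the graph.
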(event `self.ReceiveTick`
  (params (DeltaSeconds :type "Float (single-precision)")))

(event `self.Interaction.OnInteract`
  (params (Character :type "BaseCharacter Object Reference"))
  (bind _asbase_player_controller (cast `BasePlayerController` (`Pawn.GetController` Character) :!pure true))
  (bind _returnvalue (`|CreateWidget` "/Game/Blueprint/UI/WBP_StorageInventory.WBP_StorageInventory_C" _asbase_player_controller self))
  (`UserWidget.AddToViewport` _returnvalue 0)
  (set `PlayerController.bShowMouseCursor` true _asbase_player_controller))

(fn `UserConstructionScript`
  (`self.InitializeComponents` (`self.Inventory`)))