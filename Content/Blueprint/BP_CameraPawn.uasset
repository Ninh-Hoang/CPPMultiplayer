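; RTS-style camera pawn that sends move orders to the player's controlled unit from cursor clicks.
; After a one-second delay at BeginPlay, it creates a flock through the AI conductor, adds each ally as a boid and sets its blackboard PlayerPawn to the controlled unit.
; Right-click issues a simple move to the traced cursor hit and Shift+right-click queues one, both drawing a debug sphere.
; Insert-order and default-allies order nodes are unconnected.
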(event `self.ReceiveBeginPlay`
  (`KismetSystemLibrary.Delay` 1.0)
  (bind (_success _returnvalue) (`self.BP_GetControlledUnit`))
  (bind _returnvalue_2 (`ARTAIConductor.CreateFlock` (`ARTGameState.GetAIConductor`)))
  (set `self.NewVar_0` _returnvalue_2)
  (for _array_element (`ARTAIConductor.GetAlliesList` (`ARTGameState.GetAIConductor`))
    (`BlackboardComponent.SetValueAsObject` (`AIBlueprintHelperLibrary.GetBlackboard` _array_element) "PlayerPawn" _returnvalue)
    (bind _returnvalue_3 (`ARTAIConductor.TryAddBoidToList` (`ARTGameState.GetAIConductor`) (`self.NewVar_0`) _array_element))
    (`KismetSystemLibrary.PrintString` (`KismetStringLibrary.Conv_BoolToString` _returnvalue_3))))

(event `Key|RightMouseButton`
  (params (Key :type "Key Structure"))
  (bind (_bblockinghit _binitialoverlap _time _distance _location _impactpoint _normal _impactnormal _physmat _hitactor) (`GameplayStatics.BreakHitResult` (`PlayerController.GetHitResultUnderCursorByChannel` (`GameplayStatics.GetPlayerController` 0) "TraceTypeQuery1" true)))
  (:`Pressed`
    (bind (_success _returnvalue) (`self.BP_GetControlledUnit`))
    (if _success
      (`ARTOrderHelper.IssueOrder` _returnvalue (make `ARTOrderData` "/Game/Blueprint/Order/OR_SimpleMove.OR_SimpleMove_C" true (`KismetMathLibrary.Conv_VectorToVector2D` _location) _hitactor))
      (`KismetSystemLibrary.PrintString` (`KismetStringLibrary.Conv_VectorToString` (`BlackboardComponent.GetValueAsVector` (`AIBlueprintHelperLibrary.GetBlackboard` (`self.GetController` _returnvalue)) "Order_Location")))
      (`KismetSystemLibrary.DrawDebugSphere` _location 30.0 12 (struct :`R` 1.0 :`G` 1.0 :`B` 1.0 :`A` 1.0) 1.0 1.0 :!label _label))))

(event `Key|Shift+RightMouseButton`
  (params (Key :type "Key Structure"))
  (bind (_bblockinghit _binitialoverlap _time _distance _location _impactpoint _normal _impactnormal _physmat _hitactor) (`GameplayStatics.BreakHitResult` (`PlayerController.GetHitResultUnderCursorByChannel` (`GameplayStatics.GetPlayerController` 0) "TraceTypeQuery1" true)))
  (:`Pressed`
    (`ARTOrderHelper.EnqueueOrder` (stale `Key|RightMouseButton` _returnvalue) (make `ARTOrderData` "/Game/Blueprint/Order/OR_SimpleMove.OR_SimpleMove_C" true (`KismetMathLibrary.Conv_VectorToVector2D` _location) _hitactor))
    (goto _label)))

(fn `UserConstructionScript`)