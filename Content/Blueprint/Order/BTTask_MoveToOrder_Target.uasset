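; Behavior tree task that moves the AI-controlled pawn to the order's target actor, read from the blackboard.
; The acceptance radius is the blackboard radius minus the target's bounding-box X extent, clamped to a small minimum.
; A successful move finishes the task with success, while a failed move aborts it.
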(event `self.ReceiveExecuteAI`
  (params (OwnerController :type "AIController Object Reference") (ControlledPawn :type "Pawn Object Reference"))
  (bind _returnvalue (`BTFunctionLibrary.GetBlackboardValueAsActor` (`self.Target`)))
  (`|AIMoveTo` OwnerController ControlledPawn (0.0 0.0 0.0) _returnvalue (`KismetMathLibrary.FClamp` (- (`BTFunctionLibrary.GetBlackboardValueAsFloat` (`self.AcceptanceRadius`)) (.x (`.BoxExtent` (`Actor.GetActorBounds` _returnvalue false true)))) 10.0 99999997952.0)
    (:`OnSuccess`
      (`self.FinishExecute` true))
    (:`OnFail`
      (`self.FinishAbort`))))