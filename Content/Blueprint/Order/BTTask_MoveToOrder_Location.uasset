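; Behavior tree task that moves the AI-controlled pawn to an order's location read from a blackboard vector key.
; It runs an AI move task with continuous goal tracking, finishing as success when the move ends and failure when the request fails.
; The blackboard acceptance radius is only printed for debugging.
; An unconnected older move node would shrink that radius by the pawn's bounds extent.
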(event `self.ReceiveExecuteAI`
  (params (OwnerController :type "AIController Object Reference") (ControlledPawn :type "Pawn Object Reference"))
  (`KismetSystemLibrary.PrintString` (`KismetStringLibrary.Conv_DoubleToString` (`BTFunctionLibrary.GetBlackboardValueAsFloat` (`self.AcceptanceRadius`))))
  (`AITask_MoveTo.AIMoveTo` OwnerController (`BTFunctionLibrary.GetBlackboardValueAsVector` (`self.Location`)) null -1.0 "Default" "Default" true false true
    (:`OnRequestFailed`
      (`self.FinishExecute` false))
    (:`OnMoveFinished`
      (`self.FinishExecute` true))))