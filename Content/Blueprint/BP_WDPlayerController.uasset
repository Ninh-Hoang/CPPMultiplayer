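; BP_WDPlayerController is a player controller that handles RTS-style unit selection.
; Left mouse press and release tell the HUD to start and stop selection, with release also printing the selected unit count.
; Custom events clear or add to the SelectedUnits array.
; An unconnected chain would group selected units into an AI Conductor flock and move them to the cursor hit, preserving their offsets from the group center.
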(event `Key|LeftMouseButton`
  (params (Key :type "Key Structure"))
  (bind _returnvalue (`self.GetHUD`))
  (:`Pressed`
    (message `/Game/Blueprint/SelectionInterface.StartSelection` _returnvalue))
  (:`Released`
    (message `/Game/Blueprint/SelectionInterface.StopSelection` _returnvalue)
    (`KismetSystemLibrary.PrintString` (`KismetStringLibrary.Conv_IntToString` (`KismetArrayLibrary.Array_Length` (`self.SelectedUnits`))))))

(event `ClearSelectedUnits`
  (`KismetArrayLibrary.Array_Clear` (`self.SelectedUnits`)))

(event `AddSelectedUnit`
  (params (Unit :type "ARTCharacterAI Object Reference (by ref)"))
  (`KismetArrayLibrary.Array_Add` (`self.SelectedUnits`) Unit))

(fn `UserConstructionScript`)