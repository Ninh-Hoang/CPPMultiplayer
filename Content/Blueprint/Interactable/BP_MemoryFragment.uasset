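; BP_MemoryFragment is a timed interactable, built like a chest, that uses GAS to track interaction and open state through its Barrel component.
; On authority, starting interaction applies GE_Interacting to itself; completion applies GE_ChestOpen from the interactor and removes the interacting effect, as does cancelling.
; Availability is blocked by matching gameplay tags.
; An async tag listener fires Open and Close on OpenTag changes, which currently only print debug strings.
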(event `Open`
  (`KismetSystemLibrary.PrintString` "Chest open" true true (struct :`G` 0.66 :`B` 1.0 :`A` 1.0) 1.0))

(event `Close`
  (`KismetSystemLibrary.PrintString` "Chest Close"))

(event `self.ReceiveBeginPlay`
  (bind (_asynctaskproxy _tag) (`AsyncTaskGameplayTagAddedRemoved.ListenForGameplayTagAddedOrRemoved` (`AbilitySystemBlueprintLibrary.GetAbilitySystemComponent` self) (`self.ListenTag`))
    (:`then`
      (set `self.ListenForTagAddRemovedTask` _asynctaskproxy))
    (:`OnTagAdded`
      (bind _returnvalue (== _tag (`self.OpenTag`)))
      (if _returnvalue
        (`self.Open`)))
    (:`OnTagRemoved`
      (if _returnvalue
        (`self.Close`)))))

(event `self.PreInteract`
  (params (InteractingActor :type "Actor Object Reference") (InteractionComponent :type "PrimitiveComponent Object Reference"))
  (bind _returnvalue (`AbilitySystemBlueprintLibrary.GetAbilitySystemComponent` self))
  (if (== InteractionComponent (`self.Barrel`))
    (`/Engine/EditorBlueprintResources/ActorMacros.Switch Has Authority`
      (:`Authority`
        (bind _returnvalue_2 (`AbilitySystemComponent.BP_ApplyGameplayEffectToSelf` _returnvalue "/Game/Blueprint/Player/Weapon/Interacting/GE_Interacting.GE_Interacting_C" 0.0 (`AbilitySystemComponent.MakeEffectContext` _returnvalue)))
        (set `self.GE_InteractionHandle` _returnvalue_2)))))

(event `self.PostInteract`
  (params (InteractingActor :type "Actor Object Reference") (InteractionComponent :type "PrimitiveComponent Object Reference"))
  (bind _returnvalue (`AbilitySystemBlueprintLibrary.GetAbilitySystemComponent` self))
  (if (== InteractionComponent (`self.Barrel`))
    (`/Engine/EditorBlueprintResources/ActorMacros.Switch Has Authority`
      (:`Authority`
        (`AbilitySystemComponent.BP_ApplyGameplayEffectToTarget` :`self` (`AbilitySystemBlueprintLibrary.GetAbilitySystemComponent` InteractingActor) :`GameplayEffectClass` "/Game/Blueprint/Interactable/GE_ChestOpen.GE_ChestOpen_C" :`Target` _returnvalue)
        (`AbilitySystemComponent.RemoveActiveGameplayEffect` _returnvalue (`self.GE_InteractionHandle`) -1)))))

(event `self.ReceiveEndPlay`
  (params (EndPlayReason :type "EEndPlayReason Enum" :default "Destroyed"))
  (bind _listenfortagaddremovedtask (`self.ListenForTagAddRemovedTask`))
  (`/Engine/EditorBlueprintResources/StandardMacros.IsValid` _listenfortagaddremovedtask
    (:`Is Valid`
      (`AsyncTaskGameplayTagAddedRemoved.EndTask` _listenfortagaddremovedtask))))

(event `self.CancelInteraction`
  (params (InteractionComponent :type "PrimitiveComponent Object Reference"))
  (if (== InteractionComponent (`self.Barrel`))
    (`AbilitySystemComponent.RemoveActiveGameplayEffect` (`AbilitySystemBlueprintLibrary.GetAbilitySystemComponent` self) (`self.GE_InteractionHandle`) -1)))

(fn `GetInteractionDuration`
  (params (InteractionComponent :type "PrimitiveComponent Object Reference"))
  (returns (ReturnValue :type "Float (double-precision)"))
  (if (== InteractionComponent (`self.Barrel`))
    (return (`self.OpenInteractionDuration`))
    (else
      (return 0.0))))

(fn `GetPostInteractSyncType`
  (params (InteractionComponent :type "PrimitiveComponent Object Reference"))
  (returns (bShouldSync :type Boolean) (Type :type "EAbilityTaskNetSyncType Enum"))
  (if (== InteractionComponent (`self.Barrel`))
    (return false "OnlyServerWait")
    (else
      (return false "OnlyServerWait"))))

(fn `GetPreInteractSyncType`
  (params (InteractionComponent :type "PrimitiveComponent Object Reference"))
  (returns (bShouldSync :type Boolean) (Type :type "EAbilityTaskNetSyncType Enum"))
  (return false "BothWait"))

(fn `IsAvailableForInteraction`
  (params (InteractionComponent :type "PrimitiveComponent Object Reference"))
  (returns (ReturnValue :type Boolean))
  (return (and (== InteractionComponent (`self.Barrel`)) (not (`GameplayTagAssetInterface.HasAnyMatchingGameplayTags` (`AbilitySystemBlueprintLibrary.GetAbilitySystemComponent` self) (`self.AvailabilityTags`))))))

(fn `UserConstructionScript`)