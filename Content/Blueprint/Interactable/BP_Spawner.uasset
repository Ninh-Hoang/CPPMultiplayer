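; Interactable spawner that spawns a BP_Stalker at a random EQS-found location around the player when opened.
; Interactions on its StaticMesh apply GE_Interacting, then GE_ChestOpen on completion, both on authority; tags also gate availability.
; An async gameplay tag listener turns OpenTag changes into Open, which runs the query and spawn without an authority check, or Close, which only prints.
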(event `Open`
  (bind _returnvalue (`EnvQueryManager.RunEQSQuery` "/Game/Blueprint/AI/EnvironmentQuery/EQS_FindSpawnLocationAroundPlayer.EQS_FindSpawnLocationAroundPlayer" self "AllMatching"))
  (add `EnvQueryInstanceBlueprintWrapper.OnQueryFinishedEvent` _returnvalue (delegate `OnQueryFinishedEvent_Event_0`)))

(event `OnQueryFinishedEvent_Event_0`
  (params (QueryInstance :type "EnvQueryInstanceBlueprintWrapper Object Reference") (QueryStatus :type "EEnvQueryStatus Enum" :default "Processing"))
  (bind _resultlocations (`EnvQueryInstanceBlueprintWrapper.GetQueryResultsAsLocations` QueryInstance))
  (`|SpawnActorFromClass` "/Game/Blueprint/AI/Stalker/BP_Stalker.BP_Stalker_C" (`KismetMathLibrary.Conv_VectorToTransform` (`KismetArrayLibrary.Array_Random` _resultlocations)) "AdjustIfPossibleButDontSpawnIfColliding" "OverrideRootScale" null null))

(event `Close`
  (`KismetSystemLibrary.PrintString` "Chest Close"))

(event `self.ReceiveBeginPlay`
  (bind (_asynctaskproxy _tag) (`AsyncTaskGameplayTagAddedRemoved.ListenForGameplayTagAddedOrRemoved` (`AbilitySystemBlueprintLibrary.GetAbilitySystemComponent` self) (`self.InteractionTag`))
    (:`then`
      (set `self.Async Task` _asynctaskproxy))
    (:`OnTagAdded`
      (bind _returnvalue (== _tag (`self.OpenTag`)))
      (if _returnvalue
        (`self.Open`)))
    (:`OnTagRemoved`
      (if _returnvalue
        (`self.Close`)))))

(event `self.PreInteract`
  (params (InteractingActor :type "Actor Object Reference") (InteractionComponent :type "PrimitiveComponent Object Reference"))
  (bind _returnvalue (`AbilitySystemBlueprintLibrary.GetAbilitySystemComponent` self))
  (if (== InteractionComponent (`self.StaticMesh`))
    (`/Engine/EditorBlueprintResources/ActorMacros.Switch Has Authority`
      (:`Authority`
        (bind _returnvalue_2 (`AbilitySystemComponent.BP_ApplyGameplayEffectToSelf` _returnvalue "/Game/Blueprint/Player/Weapon/Interacting/GE_Interacting.GE_Interacting_C" 0.0 (`AbilitySystemComponent.MakeEffectContext` _returnvalue)))
        (set `self.GE Interaction Handle` _returnvalue_2)))))

(event `self.PostInteract`
  (params (InteractingActor :type "Actor Object Reference") (InteractionComponent :type "PrimitiveComponent Object Reference"))
  (bind _returnvalue (`AbilitySystemBlueprintLibrary.GetAbilitySystemComponent` self))
  (if (== InteractionComponent (`self.StaticMesh`))
    (`/Engine/EditorBlueprintResources/ActorMacros.Switch Has Authority`
      (:`Authority`
        (`AbilitySystemComponent.BP_ApplyGameplayEffectToTarget` :`self` (`AbilitySystemBlueprintLibrary.GetAbilitySystemComponent` InteractingActor) :`GameplayEffectClass` "/Game/Blueprint/Interactable/GE_ChestOpen.GE_ChestOpen_C" :`Target` _returnvalue)
        (`AbilitySystemComponent.RemoveActiveGameplayEffect` _returnvalue (`self.GE Interaction Handle`) -1)))))

(event `self.ReceiveEndPlay`
  (params (EndPlayReason :type "EEndPlayReason Enum" :default "Destroyed"))
  (bind _async_task (`self.Async Task`))
  (`/Engine/EditorBlueprintResources/StandardMacros.IsValid` _async_task
    (:`Is Valid`
      (`AsyncTaskGameplayTagAddedRemoved.EndTask` _async_task))))

(event `self.CancelInteraction`
  (params (InteractionComponent :type "PrimitiveComponent Object Reference"))
  (if (== InteractionComponent (`self.StaticMesh`))
    (`AbilitySystemComponent.RemoveActiveGameplayEffect` (`AbilitySystemBlueprintLibrary.GetAbilitySystemComponent` self) (`self.GE Interaction Handle`) -1)))

(fn `GetInteractionDuration`
  (params (InteractionComponent :type "PrimitiveComponent Object Reference"))
  (returns (ReturnValue :type "Float (double-precision)"))
  (return (`self.InteractionDuration`)))

(fn `GetPostInteractSyncType`
  (params (InteractionComponent :type "PrimitiveComponent Object Reference"))
  (returns (bShouldSync :type Boolean) (Type :type "EAbilityTaskNetSyncType Enum"))
  (return false "BothWait"))

(fn `GetPreInteractSyncType`
  (params (InteractionComponent :type "PrimitiveComponent Object Reference"))
  (returns (bShouldSync :type Boolean) (Type :type "EAbilityTaskNetSyncType Enum"))
  (return false "BothWait"))

(fn `IsAvailableForInteraction`
  (params (InteractionComponent :type "PrimitiveComponent Object Reference"))
  (returns (ReturnValue :type Boolean))
  (return (and (== InteractionComponent (`self.StaticMesh`)) (not (`GameplayTagAssetInterface.HasAnyMatchingGameplayTags` (`AbilitySystemBlueprintLibrary.GetAbilitySystemComponent` self) (`self.Tag Container`))))))

(fn `UserConstructionScript`)